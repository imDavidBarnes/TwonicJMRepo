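; Blueprint for a pattern puzzle where the player must enter four pillar trigger boxes in green, yellow, red, blue order.
; A counter tracks progress: later pillars reset it when out of order, while green always restarts it at one.
; Completing the order destroys the triggers, plays a completion sequence and spawns a vase at the spawn cube, marked as a placeholder reward.
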(event `Reset Puzzle`
  ;[1 1 1] Pattern_Puzzle (Joel M, assisted by David B )
  (set `self.PillarCount` 0))

(event `self.GreenPillar_TriggerBox.OnComponentBeginOverlap`
  (params (OverlappedComponent :type "PrimitiveComponent Object Reference") (OtherActor :type "Actor Object Reference") (OtherComp :type "PrimitiveComponent Object Reference") (OtherBodyIndex :type Integer) (bFromSweep :type Boolean) (SweepResult :type "HitResult Structure (by ref)"))
  ;[1 1 1] Pattern_Puzzle (Joel M, assisted by David B )
  (cast `/Game/Blueprints/Character/BP_Player` OtherActor)
  (if (>= (`self.PillarCount`) 0)
    (set `self.PillarCount` 1)
    (`KismetSystemLibrary.PrintString` "GREEN ON")
    (else
      (`self.Reset Puzzle`))))

(event `self.YellowPillar_TriggerBox.OnComponentBeginOverlap`
  (params (OverlappedComponent :type "PrimitiveComponent Object Reference") (OtherActor :type "Actor Object Reference") (OtherComp :type "PrimitiveComponent Object Reference") (OtherBodyIndex :type Integer) (bFromSweep :type Boolean) (SweepResult :type "HitResult Structure (by ref)"))
  ;[1 1 1] Pattern_Puzzle (Joel M, assisted by David B )
  (cast `/Game/Blueprints/Character/BP_Player` OtherActor)
  (if (== (`self.PillarCount`) 1)
    (set `self.PillarCount` 2)
    (`KismetSystemLibrary.PrintString` "YELLOW ON")
    (else
      (`self.Reset Puzzle`))))

(event `self.RedPillar_TriggerBox.OnComponentBeginOverlap`
  (params (OverlappedComponent :type "PrimitiveComponent Object Reference") (OtherActor :type "Actor Object Reference") (OtherComp :type "PrimitiveComponent Object Reference") (OtherBodyIndex :type Integer) (bFromSweep :type Boolean) (SweepResult :type "HitResult Structure (by ref)"))
  ;[1 1 1] Pattern_Puzzle (Joel M, assisted by David B )
  (cast `/Game/Blueprints/Character/BP_Player` OtherActor)
  (if (== (`self.PillarCount`) 2)
    (set `self.PillarCount` 3)
    (`KismetSystemLibrary.PrintString` "RED ON")
    (else
      (`self.Reset Puzzle`))))

(event `self.BluePillar_TriggerBox.OnComponentBeginOverlap`
  (params (OverlappedComponent :type "PrimitiveComponent Object Reference") (OtherActor :type "Actor Object Reference") (OtherComp :type "PrimitiveComponent Object Reference") (OtherBodyIndex :type Integer) (bFromSweep :type Boolean) (SweepResult :type "HitResult Structure (by ref)"))
  (bind _returnvalue_location (`KismetMathLibrary.BreakTransform` (`SceneComponent.K2_GetComponentToWorld` (`self.SpawnCube`))))
  ;[1 1 1] Pattern_Puzzle (Joel M, assisted by David B )
  (cast `/Game/Blueprints/Character/BP_Player` OtherActor)
  (if (== (`self.PillarCount`) 3)
    (set `self.PillarCount` 4)
    (`KismetSystemLibrary.PrintString` "BLUE ON, PUZZLE COMPLETE")
    (`ActorComponent.K2_DestroyComponent` (`self.BluePillar_TriggerBox`))
    (`ActorComponent.K2_DestroyComponent` (`self.GreenPillar_TriggerBox`))
    (`ActorComponent.K2_DestroyComponent` (`self.RedPillar_TriggerBox`))
    (`ActorComponent.K2_DestroyComponent` (`self.YellowPillar_TriggerBox`))
    (`MovieSceneSequencePlayer.Play` (`ActorSequenceComponent.SequencePlayer` (`self.Pattern_Puzzle_Complete_Ani`)))
    ;[1 1 1] REPACE WITH CORRECT ITEM
    (`|SpawnActorFromClass` "/Game/Blueprints/OverworldObjects/BP_Vase.BP_Vase_C" (`KismetMathLibrary.MakeTransform` _returnvalue_location) "Undefined" "OverrideRootScale" null null)
    (else
      (`self.Reset Puzzle`))))

(fn `UserConstructionScript`)