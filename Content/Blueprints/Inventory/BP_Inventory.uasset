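; BP_Inventory is the inventory actor, which stores items and pauses gameplay through StopGame and ContinueGame.
; Items is a map edited by AddItem and RemoveItem, with debug prints.
; StopGame moves input from BP_Player to this actor, shows the cursor and disables player and MainEnemyPawn movement; ContinueGame reverses this, restoring walking.
; Its ShowInven key asks BP_Player to remove the inventory UI and clears IsShowing.
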(event `InputAction|ShowInven`
  (params (Key :type "Key Structure"))
  ;[1 1 1] Remove inventory from UI - Patrick Devine
  (:`Pressed`
    (bind _asbp_player (cast `/Game/Blueprints/Character/BP_Player` (`GameplayStatics.GetPlayerPawn` 0)))
    (`/Game/Blueprints/Character/BP_Player.Remove Inventory` _asbp_player)
    (set `self.isShowing` false)))

(event `TurnOnPlayerInput`
  (bind _returnvalue (`GameplayStatics.GetPlayerController` 0))
  ;[1 1 1] Make sure player can't dodge or attack - Patrick Devine
  (bind _asbp_player (cast `/Game/Blueprints/Character/BP_Player` (`GameplayStatics.GetPlayerPawn` 0)))
  (`self.EnableInput` _asbp_player _returnvalue)
  (`self.DisableInput` _returnvalue))

(event `TurnOffPlayerInput`
  (bind _returnvalue (`GameplayStatics.GetPlayerController` 0))
  ;[1 1 1] Make sure player can't dodge or attack - Patrick Devine
  (bind _asbp_player (cast `/Game/Blueprints/Character/BP_Player` (`GameplayStatics.GetPlayerPawn` 0)))
  (`self.DisableInput` _asbp_player _returnvalue)
  (`self.EnableInput` _returnvalue))

(event `StopGame`
  ;[1 1 1] Inven HUD
  (`KismetSystemLibrary.PrintString` "Stop Game Call")
  (`self.TurnOffPlayerInput`)
  (`CharacterMovementComponent.DisableMovement` (`Character.CharacterMovement` (`GameplayStatics.GetPlayerCharacter` 0)))
  (set `PlayerController.bShowMouseCursor` true (`GameplayStatics.GetPlayerController` 0))
  (bind _outactors (`GameplayStatics.GetAllActorsOfClass` "/Game/Blueprints/EnemyAI/MainEnemyPawn.MainEnemyPawn_C"))
  (for _array_element _outactors
    (`CharacterMovementComponent.DisableMovement` (`Character.CharacterMovement` _array_element))))

(event `ContinueGame`
  ;[1 1 1] Inven HUD
  (`KismetSystemLibrary.PrintString` "Continue Game Call")
  (set `PlayerController.bShowMouseCursor` false (`GameplayStatics.GetPlayerController` 0))
  (`self.TurnOnPlayerInput`)
  (`CharacterMovementComponent.SetMovementMode` (`Character.CharacterMovement` (`GameplayStatics.GetPlayerCharacter` 0)) "MOVE_Walking" 0)
  (bind _outactors (`GameplayStatics.GetAllActorsOfClass` "/Game/Blueprints/EnemyAI/MainEnemyPawn.MainEnemyPawn_C"))
  (for _array_element _outactors
    (`CharacterMovementComponent.SetMovementMode` (`Character.CharacterMovement` _array_element) "MOVE_Walking" 0)))

(fn `AddItem`
  (params (pickup :type "Pickup Class Reference") (AddItem :type Name))
  (bind _items (`self.items`))
  (`BlueprintMapLibrary.Map_Add` _items AddItem pickup)
  (if (`.ReturnValue` (`BlueprintMapLibrary.Map_Find` _items AddItem))
    (`KismetSystemLibrary.PrintString` (`KismetStringLibrary.Concat_StrStr` (`KismetStringLibrary.Conv_NameToString` AddItem) " was added to inven") true true (struct :`R` 0.337497 :`G` 1.0 :`B` 0.411363 :`A` 1.0))
    (else
      (`KismetSystemLibrary.PrintString` "failed to add" true true (struct :`R` 1.0 :`G` 0.266788 :`B` 0.217016 :`A` 1.0)))))

(fn `RemoveItem`
  (params (pickup :type Name))
  (bind _items (`self.items`))
  (if (`.ReturnValue` (`BlueprintMapLibrary.Map_Find` _items pickup))
    (bind _returnvalue (`BlueprintMapLibrary.Map_Remove` _items pickup))
    (if _returnvalue
      (`KismetSystemLibrary.PrintString` (`KismetStringLibrary.Concat_StrStr` (`KismetStringLibrary.Conv_NameToString` pickup) " was removed") true true (struct :`R` 0.337497 :`G` 1.0 :`B` 0.411363 :`A` 1.0))
      (else
        (`KismetSystemLibrary.PrintString` "failed to remove" true true (struct :`R` 1.0 :`G` 0.266788 :`B` 0.217016 :`A` 1.0))))
    (else
      (`KismetSystemLibrary.PrintString` "item not found"))))

(fn `UserConstructionScript`)