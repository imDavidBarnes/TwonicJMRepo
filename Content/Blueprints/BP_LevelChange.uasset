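; BP_LevelChange is a trigger volume that moves the player to another level named by LevelName.
; When a PlayerCharacter first overlaps the box, it saves the player's health and inventory to BP_GameInstance, flagged as loaded from another level.
; If the origin is the overworld, it also stores the RespawnLocation position.
; After a short delay it opens the target level.
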(event `self.Box.OnComponentBeginOverlap`
  (params (OverlappedComponent :type "PrimitiveComponent Object Reference") (OtherActor :type "Actor Object Reference") (OtherComp :type "PrimitiveComponent Object Reference") (OtherBodyIndex :type Integer) (bFromSweep :type Boolean) (SweepResult :type "HitResult Structure (by ref)"))
  (bind _returnvalue_location (`KismetMathLibrary.BreakTransform` (`SceneComponent.K2_GetComponentToWorld` (`self.RespawnLocation`))))
  ;[1 0.02144 0.4325] When Level Loads Save Data to Game Instance - David Barnes
  (cast `PlayerCharacter` OtherActor)
  (`/Engine/EditorBlueprintResources/StandardMacros.DoOnce` false
    (:`Completed`
      (bind _asbp_game_instance (cast `/Game/Blueprints/BP_GameInstance` (`GameplayStatics.GetGameInstance`)))
      (if (`self.IsOriginOverworld`)
        (`/Game/Blueprints/BP_GameInstance.SaveOverworldLocation` _asbp_game_instance _returnvalue_location))
      (bind _asbp_player (cast `/Game/Blueprints/Character/BP_Player` (`GameplayStatics.GetPlayerCharacter` 0)))
      (bind _returnvalue (`PlayerCharacter.GetHealth` _asbp_player))
      (`/Game/Blueprints/BP_GameInstance.SaveDataForLevelLoad` _asbp_game_instance _returnvalue true (`/Game/Blueprints/Character/BP_Player.InventoryItems` _asbp_player))
      (`KismetSystemLibrary.Delay` 0.5)
      (`GameplayStatics.OpenLevel` (`self.Level Name`)))))

(fn `UserConstructionScript`)