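; Projectile actor that moves along its spawn forward vector by teleporting each Tick, with collision briefly disabled and destruction on a timer.
; Overlaps skip ignored classes and other projectiles, and hurt the owner only after a parry.
; A parrying player reverses its horizontal direction.
; Other valid hits trigger an explosion that stops the projectile, enlarges a proximity sphere and applies damage, with an AOE flag controlling repeat damage.
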(event `self.ReceiveBeginPlay`
  ;[1 1 1] Destroy actor after five seconds, turn on collision after 0.2 seconds
  (set `self.HasBeenParried` false)
  (`KismetSystemLibrary.Delay` 0.2)
  (`self.SetActorEnableCollision` true)
  (`KismetSystemLibrary.Delay` 5.0)
  (`self.K2_DestroyActor`))

(event `self.ReceiveTick`
  (params (DeltaSeconds :type "Float (single-precision)"))
  ;[1 1 1] Move projectile forward - Patrick & Keiran
  (`self.K2_TeleportTo` (+ (`self.K2_GetActorLocation`) (* (`self.MoveVector`) (`self.Speed`))) (`self.K2_GetActorRotation`)))

(event `self.ReceiveActorBeginOverlap`
  (params (OtherActor :type "Actor Object Reference"))
  (bind (_movevector_x _movevector_y _movevector_z) (`KismetMathLibrary.BreakVector` (`self.MoveVector`)))
  (bind (_returnvalue_x _returnvalue_y) (`KismetMathLibrary.BreakVector` (* (`self.MoveVector`) -1.0)))
  ;[1 1 1] Event overlap (on collision destroy self)
  (bind _shouldignore (`self.FindIfIgnore` OtherActor))
  (if (not _shouldignore)
    (cast `/Game/Blueprints/BP_Projectile` OtherActor
      (:`CastFailed`
        ;;[1 1 1] If parried send in other direction - Patrick Devine
        (if (== OtherActor (`self.GetOwner`))
          (if (`self.HasBeenParried`)
            (`self.DealDamage` OtherActor))
          (else
            (bind _asbp_player (cast `/Game/Blueprints/Character/BP_Player` (`GameplayStatics.GetPlayerPawn` 0))
              (:`then`
                (if (and (`/Game/Blueprints/Character/BP_Player.IsParrying` _asbp_player) (== OtherActor _asbp_player))
                  (set `self.MoveVector` (`KismetMathLibrary.MakeVector` _returnvalue_x _returnvalue_y _movevector_z))
                  (set `self.HasBeenParried` true)
                  (else
                    (`self.DealDamage` OtherActor :!label _label))))
              (:`CastFailed`
                (goto _label)))))))))

(event `self.ReceiveHit`
  (params (MyComp :type "PrimitiveComponent Object Reference") (Other :type "Actor Object Reference") (OtherComp :type "PrimitiveComponent Object Reference") (bSelfMoved :type Boolean) (HitLocation :type "Vector Structure") (HitNormal :type "Vector Structure") (NormalImpulse :type "Vector Structure") (Hit :type "HitResult Structure (by ref)"))
  ;[1 1 1] Event overlap (on collision destroy self)
)

(event `DealDamage`
  (params (Actor :type "Actor Object Reference"))
  ;[1 1 1] Event overlap (on collision destroy self)
  (`self.Explode`)
  (if (`self.CanDamage`)
    (if (not (`self.IsAOE`))
      (`/Engine/EditorBlueprintResources/StandardMacros.DoOnce` false
        (:`Completed`
          _)))
    (`GameplayStatics.ApplyDamage` Actor (`self.Damage`) null self)))

(event `Explode`
  (bind _sphere (`self.Sphere`))
  ;[1 1 1] Increase size of prox sphere for explosion effect - Patrick Devine
  (`SphereComponent.SetSphereRadius` (`self.Sphere1`) (`self.ExplosionProxRadius`) true)
  (set `self.CanDamage` true)
  (`SceneComponent.SetVisibility` _sphere false false)
  (`PrimitiveComponent.SetCollisionEnabled` _sphere "NoCollision")
  (set `self.Speed` 0.0))

(fn `FindIfIgnore`
  (params (InActor :type "Actor Object Reference"))
  (returns (ShouldIgnore :type Boolean))
  (locals (Ignore :type Boolean))
  (set `local.Ignore` false)
  (for _array_element (`self.IgnoreList`)
    (if (== _array_element (`GameplayStatics.GetObjectClass` InActor))
      (set `local.Ignore` true)))
  (return (`local.Ignore`)))

(fn `UserConstructionScript`
  ;[1 1 1] Spawn projectile and move to starting pos (disable collision) - Patrick & Keiran
  (bind _output_get (set `self.MoveVector` (`self.GetActorForwardVector`)))
  (`self.K2_TeleportTo` (+ _output_get (`self.K2_GetActorLocation`)) (`self.K2_GetActorRotation`))
  (`self.SetActorEnableCollision` false))