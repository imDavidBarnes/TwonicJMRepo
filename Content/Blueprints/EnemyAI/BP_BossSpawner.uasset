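; BP_BossSpawner is an interactable, single-use spawner that creates an enemy, presumably a boss, when the player triggers it.
; Input on the actor is disabled at BeginPlay and enabled only while BP_Player overlaps ProxSphere, gating the Interact action by proximity.
; Pressing Interact calls SpawnEnemy, which is not defined in this graph, with a fixed uniform vector, then destroys the spawner.
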(event `self.ReceiveBeginPlay`
  (`self.DisableInput` (`GameplayStatics.GetPlayerController` 0)))

(event `self.ProxSphere.OnComponentBeginOverlap`
  (params (OverlappedComponent :type "PrimitiveComponent Object Reference") (OtherActor :type "Actor Object Reference") (OtherComp :type "PrimitiveComponent Object Reference") (OtherBodyIndex :type Integer) (bFromSweep :type Boolean) (SweepResult :type "HitResult Structure (by ref)"))
  (cast `/Game/Blueprints/Character/BP_Player` OtherActor)
  (`self.EnableInput` (`GameplayStatics.GetPlayerController` 0)))

(event `self.ProxSphere.OnComponentEndOverlap`
  (params (OverlappedComponent :type "PrimitiveComponent Object Reference") (OtherActor :type "Actor Object Reference") (OtherComp :type "PrimitiveComponent Object Reference") (OtherBodyIndex :type Integer))
  (cast `/Game/Blueprints/Character/BP_Player` OtherActor)
  (`self.DisableInput` (`GameplayStatics.GetPlayerController` 0)))

(event `InputAction|Interact`
  (params (Key :type "Key Structure"))
  (:`Pressed`
    (`self.Spawn Enemy` (2.5 2.5 2.5))
    (`self.K2_DestroyActor`)))

(fn `UserConstructionScript`
  (`parent.UserConstructionScript`))