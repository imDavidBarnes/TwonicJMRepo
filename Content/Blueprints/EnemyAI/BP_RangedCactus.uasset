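; BP_RangedCactus is a ranged cactus enemy that fires spike projectiles at the player.
; Each tick it faces the player, runs an attack sense check and calls EnemyAttack while in range.
; A DoOnce gates the attack, which, unless staggered, spawns a half-scale BP_CactusSpike rotated toward the player.
; ResetAttack reopens the gate after a random delay, but only runs after a spike spawns.
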(event `self.ReceiveBeginPlay`
  (`parent.ReceiveBeginPlay`))

(event `self.ReceiveTick`
  (params (DeltaSeconds :type "Float (single-precision)"))
  (`self.Face Player`)
  (`self.AttackSense` (`self.Range`))
  (if (`self.InRange`)
    (bind _toplayer (`self.GetToPlayer`))
    (`self.EnemyAttack` _toplayer 1.0)))

(event `self.EnemyAttack`
  (params (ToPlayer :type "Vector Structure") (Scale :type "Float (single-precision)"))
  (bind _returnvalue (`self.K2_GetActorLocation`))
  (`/Engine/EditorBlueprintResources/StandardMacros.DoOnce` false :!label _label
    (:`Completed`
      (if (not (`self.Staggered`))
        (bind _asbp_player (cast `/Game/Blueprints/Character/BP_Player` (`GameplayStatics.GetPlayerPawn` 0)))
        (`|SpawnActorFromClass` "/Game/Blueprints/EnemyAI/EnemyProjectileAttacks/BP_CactusSpike.BP_CactusSpike_C" (`KismetMathLibrary.MakeTransform` _returnvalue (`KismetMathLibrary.FindLookAtRotation` _returnvalue (`self.K2_GetActorLocation` _asbp_player)) (0.5 0.5 0.5)) "AlwaysSpawn" "OverrideRootScale" null null)
        (`self.Reset Attack`)))))

(event `Reset Attack`
  (`KismetSystemLibrary.Delay` (`KismetMathLibrary.RandomFloatInRange` 2.0 5.0))
  (goto _label :!via `Reset`))

(fn `UserConstructionScript`
  (`parent.UserConstructionScript`))