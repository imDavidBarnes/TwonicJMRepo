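; Enemy cactus Blueprint meant to roll while moving and face the player when stopped, adding to inherited parent behavior.
; Roll advances an angle into actor pitch while keeping yaw, and StopRolling resets rotation and calls FacePlayer.
; The logic that compares position with OldPos to pick either event and pins TargetSelecter to the capsule base is disconnected, so Tick only runs the parent's.
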(event `self.ReceiveBeginPlay`
  (`parent.ReceiveBeginPlay`)
  (set `self.OldPos` (`self.K2_GetActorLocation`)))

(event `self.ReceiveTick`
  (params (DeltaSeconds :type "Float (single-precision)"))
  ;[1 1 1] Cactus move - Patrick Devine
  (`parent.ReceiveTick` DeltaSeconds))

(event `Roll`
  (bind (_returnvalue_roll _returnvalue_pitch _returnvalue_yaw) (`KismetMathLibrary.BreakRotator` (`self.K2_GetActorRotation`)))
  (bind _yrotation (`self.YRotation`))
  ;[1 1 1] Rolls cactus on move - Patrick Devine
  (set `self.YRotation` (+ _yrotation (* (`self.YIncrement`) (`self.DeltaTime`))))
  (if (>= _yrotation 360.0)
    (set `self.YRotation` 0.0)
    (else
      (`self.K2_SetActorRotation` (`KismetMathLibrary.MakeRotator` 0.0 (- 360.0 (`self.YRotation`)) _returnvalue_yaw)))))

(event `StopRolling`
  ;[1 1 1] Rolls cactus on move - Patrick Devine
  (`self.K2_SetActorRotation` (`KismetMathLibrary.MakeRotator` 0.0))
  (`self.Face Player`))

(fn `UserConstructionScript`
  (`parent.UserConstructionScript`))