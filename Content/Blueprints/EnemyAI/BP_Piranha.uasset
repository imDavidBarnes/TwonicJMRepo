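; Piranha enemy character that leaps at the player's position and drops away after the attack.
; ResetJump re-arms a DoOnce that snapshots a point above the player, the distance and facing.
; Tick relaunches it along that fixed vector until it horizontally nears the saved location, then disables capsule collision and launches it downward.
; Hitting the player also disables collision and ends the attack, recoiling it up and away.
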(event `self.ReceiveBeginPlay`
  ;[1 1 1] Init values Piranha - Patrick Devine
  (`parent.ReceiveBeginPlay`)
  (`self.Start Patroling`)
  (`self.GetPlayerDir`)
  (`self.Reset Jump`))

(event `Reset Jump`
  ;[1 1 1] Piranha jump - Patrick Devine
  (set `self.CanAttack` true)
  (goto _label :!via `Reset`))

(event `self.ReceiveTick`
  (params (DeltaSeconds :type "Float (single-precision)"))
  (bind (_returnvalue_x _returnvalue_y) (`KismetMathLibrary.BreakVector` (* (`KismetMathLibrary.Normal` (`self.ToPlayer`)) (`self.DistanceToPlayer`))))
  ;[1 1 1] Piranha jump - Patrick Devine
  (`self.Below Level`)
  (`|ExecutionSequence`
    (:`then_0`
      (`/Engine/EditorBlueprintResources/StandardMacros.DoOnce` false :!label _label
        (:`Completed`
          (`self.GetPlayerDir`)
          (set `self.DistanceToPlayer` (`KismetMathLibrary.VSize` (`self.ToPlayer`)))
          (`self.Face Player`))))
    (:`then_1`
      (if (`self.CanAttack`)
        (`self.LaunchCharacter` (* (`KismetMathLibrary.Normal` (`self.ToPlayer`)) (`self.DistanceToPlayer`)) true true)
        (if (<= (`KismetMathLibrary.VSizeXY` (- (`self.MoveLoc`) (`self.K2_GetActorLocation`))) 25.0)
          (`PrimitiveComponent.SetCollisionEnabled` (`self.CapsuleComponent`) "NoCollision")
          (set `self.CanAttack` false)
          (`self.LaunchCharacter` (`KismetMathLibrary.MakeVector` _returnvalue_x _returnvalue_y (* -1 (`self.LaunchDist`))) true true))))))

(event `self.ReceiveHit`
  (params (MyComp :type "PrimitiveComponent Object Reference") (Other :type "Actor Object Reference") (OtherComp :type "PrimitiveComponent Object Reference") (bSelfMoved :type Boolean) (HitLocation :type "Vector Structure") (HitNormal :type "Vector Structure") (NormalImpulse :type "Vector Structure") (Hit :type "HitResult Structure (by ref)"))
  (bind _launchdist (`self.LaunchDist`))
  (bind (_returnvalue_x _returnvalue_y) (`KismetMathLibrary.BreakVector` (* (`KismetMathLibrary.Normal` (* (`self.ToPlayer`) -1.0)) _launchdist)))
  ;[1 1 1] Recoil from attack - Patrick Devine
  (`self.Parent Hit` Other)
  (cast `/Game/Blueprints/Character/BP_Player` Other)
  (`PrimitiveComponent.SetCollisionEnabled` (`self.CapsuleComponent`) "NoCollision")
  (`self.LaunchCharacter` (`KismetMathLibrary.MakeVector` _returnvalue_x _returnvalue_y _launchdist) true true)
  (set `self.CanAttack` false))

(fn `GetPlayerDir`
  (bind _asbp_player (cast `/Game/Blueprints/Character/BP_Player` (`GameplayStatics.GetPlayerPawn` 0)))
  (bind (_returnvalue_x _returnvalue_y _returnvalue_z) (`KismetMathLibrary.BreakVector` (`self.K2_GetActorLocation` _asbp_player)))
  (set `self.ToPlayer` (- (`KismetMathLibrary.MakeVector` _returnvalue_x _returnvalue_y (+ _returnvalue_z 100.0)) (`self.K2_GetActorLocation`)))
  (set `self.MoveLoc` (`KismetMathLibrary.MakeVector` _returnvalue_x _returnvalue_y _returnvalue_z)))

(fn `UserConstructionScript`
  (`parent.UserConstructionScript`))