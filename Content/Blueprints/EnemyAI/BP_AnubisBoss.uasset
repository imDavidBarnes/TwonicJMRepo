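; Anubis boss enemy AI that faces the player and alternates between a chase-to-melee attack and a fireball attack.
; A Do Once on Tick, re-armed after a random delay, makes a weighted pick favoring melee in extended range and fireballs otherwise.
; Melee chases until in range, while fireballs spawn only within a wider range check.
; Inherited sensing, facing and attack functions do the work, and Tick hides the enemy HUD.
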(event `GoToPlayer`
  ;[1 1 1] Walk to player - Patrick Devine
  (bind _asbp_player (cast `/Game/Blueprints/Character/BP_Player` (`GameplayStatics.GetPlayerPawn` 0)))
  (`|AIMoveTo` self (0.0 0.0 0.0) _asbp_player))

(event `FireProjectile`
  ;[1 1 1] Firing fire ball - Patrick Devine
  (`self.AttackSense` (* (`self.Range`) 4.0))
  (if (`self.InRange`)
    (`|SpawnActorFromClass` "/Game/Blueprints/EnemyAI/EnemyProjectileAttacks/BP_FireAttack.BP_FireAttack_C" (`KismetMathLibrary.MakeTransform` (`self.K2_GetActorLocation`) (`self.K2_GetActorRotation`) (0.5 0.5 0.5)) "AlwaysSpawn" "OverrideRootScale" self null)
    (`KismetSystemLibrary.Delay` 2.0)
    (`self.Reset Attack Rand`)
    (else
      (`self.Reset Attack Rand`))))

(event `self.ReceiveBeginPlay`
  (`parent.ReceiveBeginPlay`)
  (set `self.CanSee` true))

(event `Initiate Attack`
  ;[1 1 1] Cycling attacks on random - Patrick Devine
  (set `self.InRange` false)
  (set `self.Attacking` true))

(event `Reset Attack Rand`
  ;[1 1 1] Cycling attacks on random - Patrick Devine
  (`KismetSystemLibrary.Delay` (`KismetMathLibrary.RandomFloatInRange` 2.5 4.0))
  (goto _label :!via `Reset`))

(event `self.ReceiveTick`
  (params (DeltaSeconds :type "Float (single-precision)"))
  (`SceneComponent.SetVisibility` (`self.EnemyHud`) false false)
  (set `self.DeltaTime` DeltaSeconds)
  (`self.AttackSense` (`self.Range`))
  (`self.Face Player`)
  (if (`self.Attacking`)
    (if (`self.InRange`)
      ;[1 1 1] Cycling attacks on random - Patrick Devine
      (bind _toplayer (`self.GetToPlayer`))
      (`self.EnemyAttack` _toplayer 2.5)
      (set `self.Attacking` false)
      (`|AIMoveTo` self (`self.K2_GetActorLocation`) null
        (:`OnSuccess`
          _)
        (:`OnFail`
          _))
      (`self.Reset Attack Rand`)
      (else
        (`self.GoToPlayer`)))
    (else
      (`/Engine/EditorBlueprintResources/StandardMacros.DoOnce` false :!label _label
        (:`Completed`
          (`self.AttackSense` (* (`self.Range`) (`self.RangeMultiplicative`)))
          (if (`self.InRange`)
            (if (`KismetMathLibrary.RandomBoolWithWeight` 0.75)
              (`self.Initiate Attack`)
              (else
                (`self.FireProjectile`)))
            (elif (`KismetMathLibrary.RandomBoolWithWeight` 0.75)
              (`self.FireProjectile`)
              (else
                (`self.Initiate Attack`)))))))))

(fn `UserConstructionScript`
  (`parent.UserConstructionScript`))