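; Snake enemy with four difficulty tiers that set damage and health multipliers, material, mesh and capsule radius on BeginPlay or wave-spawner change.
; Non-boss tiers use the parent Tick.
; A Boss that sees the player faces them and recursively rerolls between firing BP_SpitAttack at double range and charging into melee, rolling again after each attack.
; Overlapping its Box deals fixed damage to the player.
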(event `GoToPlayer`
  ;[1 1 1] Walk to player - Patrick Devine
  (bind _asbp_player (cast `/Game/Blueprints/Character/BP_Player` (`GameplayStatics.GetPlayerPawn` 0)))
  (`|AIMoveTo` self (0.0 0.0 0.0) _asbp_player))

(event `FireProjectile`
  ;[1 1 1] Boss tick - Patrick Devine
  (`self.AttackSense` (* (`self.Range`) 2.0))
  (if (`self.InRange`)
    (`|SpawnActorFromClass` "/Game/Blueprints/EnemyAI/EnemyProjectileAttacks/BP_SpitAttack.BP_SpitAttack_C" (`KismetMathLibrary.MakeTransform` (`self.K2_GetActorLocation`) (`self.K2_GetActorRotation`) (0.2 0.2 0.2)) "AlwaysSpawn" "OverrideRootScale" self null)
    (`KismetSystemLibrary.Delay` 2.0)
    (`self.Reset Attack Rand`)
    (else
      (`self.Reset Attack Rand`))))

(event `Reset Attack Rand`
  (bind _returnvalue (`KismetMathLibrary.RandomIntegerInRange` 0 100))
  ;[1 1 1] Boss tick - Patrick Devine
  (goto _label :!via `Reset`))

(event `self.ReceiveTick`
  (params (DeltaSeconds :type "Float (single-precision)"))
  (bind _returnvalue (`KismetMathLibrary.RandomIntegerInRange` 0 100))
  ;[1 1 1] Boss tick - Patrick Devine
  (if (and (`|EnumEquality` (`self.DifficultySnake`) "NewEnumerator3") (`self.CanSee`))
    (set `self.DeltaTime` DeltaSeconds)
    (`self.AttackSense` (`self.Range`))
    (`self.Face Player`)
    (if (`self.Attacking`)
      (if (`self.InRange`)
        (bind _toplayer (`self.GetToPlayer`))
        (`self.EnemyAttack` _toplayer 1.0)
        (set `self.Attacking` false)
        (`|AIMoveTo` self (`self.K2_GetActorLocation`) null
          (:`OnSuccess`
            _)
          (:`OnFail`
            _))
        (`self.Reset Attack Rand`))
      (else
        (`/Engine/EditorBlueprintResources/StandardMacros.DoOnce` false :!label _label
          (:`Completed`
            (if (== _returnvalue 0)
              (`self.FireProjectile`)
              (elif (== _returnvalue 100)
                (`self.Initiate Attack`)
                (else
                  (`self.Reset Attack Rand`))))))))
    (else
      (`self.Parent Tick` DeltaSeconds))))

(event `Initiate Attack`
  ;[1 1 1] Boss tick - Patrick Devine
  (set `self.InRange` false)
  (set `self.Attacking` true)
  (`self.GoToPlayer`))

(event `self.ReceiveBeginPlay`
  ;[1 1 1] Set snake difficulty level - Patrick Devine
  (`parent.ReceiveBeginPlay`)
  (`KismetSystemLibrary.Delay` 0.1)
  (`|ExecutionSequence` :!label _label_2
    (:`then_0`
      (switch `/Game/Blueprints/EnemyAI/E_Difficulty` (`self.DifficultySnake`)
        (:`NewEnumerator0`
          (`self.SetDifficultyValues` 0.5 25.0 "/Game/Materials/Mat_Green.Mat_Green")
          (`SkinnedMeshComponent.SetSkinnedAssetAndUpdate` (`self.Mesh`) "/Game/Character/Models/Snake/small_snake_retopo.small_snake_retopo" true)
          (`CapsuleComponent.SetCapsuleRadius` (`self.CapsuleComponent`) 34.0 true))
        (:`NewEnumerator1`
          (`self.SetDifficultyValues` 1.5 50.0 "/Game/Materials/Mat_Red.Mat_Red")
          (`SkinnedMeshComponent.SetSkinnedAssetAndUpdate` (`self.Mesh`) "/Game/Character/Models/Snake/small_snake_retopo.small_snake_retopo" true)
          (`CapsuleComponent.SetCapsuleRadius` (`self.CapsuleComponent`) 34.0 true))
        (:`NewEnumerator2`
          (`self.SetDifficultyValues` 2.5 75.0 "/Game/Materials/Mat_Black.Mat_Black")
          (`SkinnedMeshComponent.SetSkinnedAssetAndUpdate` (`self.Mesh`) "/Game/Character/Models/Snake/small_snake_retopo.small_snake_retopo" true)
          (`CapsuleComponent.SetCapsuleRadius` (`self.CapsuleComponent`) 34.0 true))
        (:`NewEnumerator3`
          (`self.SetDifficultyValues` 3.5 200.0 "/Game/Materials/Mat_Black.Mat_Black")
          (`SkinnedMeshComponent.SetSkinnedAssetAndUpdate` (`self.Mesh`) "/Game/Character/Models/KingCobra/g7_snake_rig.g7_snake_rig" true)
          (`CapsuleComponent.SetCapsuleRadius` (`self.CapsuleComponent`) 88.0 true))))
    (:`then_1`
      (`self.CreateHUD`)
      (`self.SetMaterial` (`self.EnemyMat`)))))

(event `ChangeDifficultyWaveSpawner`
  ;[1 1 1] Set snake difficulty level - Patrick Devine
  (goto _label_2))

(event `self.Box.OnComponentBeginOverlap`
  (params (OverlappedComponent :type "PrimitiveComponent Object Reference") (OtherActor :type "Actor Object Reference") (OtherComp :type "PrimitiveComponent Object Reference") (OtherBodyIndex :type Integer) (bFromSweep :type Boolean) (SweepResult :type "HitResult Structure (by ref)"))
  (bind _asbp_player (cast `/Game/Blueprints/Character/BP_Player` OtherActor))
  (`GameplayStatics.ApplyDamage` _asbp_player 3.5 null self))

(fn `UserConstructionScript`
  (`parent.UserConstructionScript`))