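; Enemy spawner that places an instance of its configured enemy class at every actor in its spawn point list.
; RespawnEnemies runs this loop, also triggered on BeginPlay when ShouldSpawnOnBegin is set, and copies the spawner's difficulty onto spawned BP_Snake enemies.
; SpawnEnemy separately spawns a single enemy above the spawner with a given scale and does not set difficulty.
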(event `RespawnEnemies`
  (for _array_element (`self.SpawnPoint`) :!label _label
    (bind _output_get (set `self.SpawnPointLocations` (`|MakeArray` (`self.GetTransform` _array_element))))
    (for _array_element_2 _output_get
      (bind _returnvalue (`|SpawnActorFromClass` (`self.EnemyToSpawn`) _array_element_2 "AdjustIfPossibleButAlwaysSpawn" "OverrideRootScale" null null))
      (bind _asbp_snake (cast `/Game/Blueprints/EnemyAI/BP_Snake` _returnvalue))
      (set `/Game/Blueprints/EnemyAI/BP_Snake.DifficultySnake` (`self.DifficultySpawner`) _asbp_snake))))

(event `self.ReceiveBeginPlay`
  (if (`self.ShouldSpawnOnBegin`)
    (goto _label)))

(event `Spawn Enemy`
  (params (Scale :type "Vector Structure"))
  (`|SpawnActorFromClass` (`self.EnemyToSpawn`) (`KismetMathLibrary.MakeTransform` (+ (`self.K2_GetActorLocation`) (0.0 0.0 250.0)) (`self.K2_GetActorRotation`) Scale) "AdjustIfPossibleButAlwaysSpawn" "OverrideRootScale" null null))

(fn `UserConstructionScript`)