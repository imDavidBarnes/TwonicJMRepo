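; Enemy spit attack projectile that poisons the player and disables sprinting for a short time.
; DealDamage explodes it and schedules destruction, then, once and if damage is allowed, stores the hit actor and starts a looping poison timer on players.
; Tick keeps the projectile on the hit actor while the timer applies small damage.
; After a few ticks it restores sprint and destroys itself.
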(event `self.ReceiveBeginPlay`
  (`parent.ReceiveBeginPlay`))

(event `self.ReceiveActorBeginOverlap`
  (params (OtherActor :type "Actor Object Reference"))
  (`parent.ReceiveActorBeginOverlap` OtherActor))

(event `Die`
  (params (Timer :type "Float (double-precision)"))
  ;[1 1 1] Spit attack - Patrick Devine
  (`KismetSystemLibrary.Delay` Timer)
  (`self.K2_DestroyActor`))

(event `self.ReceiveTick`
  (params (DeltaSeconds :type "Float (single-precision)"))
  (bind _hitactor (`self.HitActor`))
  ;[1 1 1] Spit attack - Patrick Devine
  (`parent.ReceiveTick` DeltaSeconds)
  (if (`KismetSystemLibrary.IsValid` _hitactor)
    (`self.K2_SetActorLocation` (`self.K2_GetActorLocation` _hitactor) false true)))

(event `self.DealDamage`
  (params (Actor :type "Actor Object Reference"))
  ;[1 1 1] Spit attack - Patrick Devine
  (`self.Die` 5.0)
  (`self.Explode`)
  (if (`self.CanDamage`)
    (`/Engine/EditorBlueprintResources/StandardMacros.DoOnce` false
      (:`Completed`
        (bind _output_get (set `self.HitActor` Actor))
        (bind _asbp_player (cast `/Game/Blueprints/Character/BP_Player` _output_get))
        (set `/Game/Blueprints/Character/BP_Player.CanSprint` false _asbp_player)
        (`KismetSystemLibrary.K2_SetTimerDelegate` (delegate `PoisonDamage`) 0.5 true 0.5)))))

(event `PoisonDamage`
  ;[1 1 1] Spit attack - Patrick Devine
  (`GameplayStatics.ApplyDamage` (`self.HitActor`) 0.2 null self)
  (bind _result (`/Engine/EditorBlueprintResources/StandardMacros.IncrementInt` (`self.HitCounter`))
    (:`  `
      (if (>= _result 5)
        (bind _asbp_player (cast `/Game/Blueprints/Character/BP_Player` (`self.HitActor`)))
        (set `/Game/Blueprints/Character/BP_Player.CanSprint` true _asbp_player)
        (`self.K2_DestroyActor`)))))

(fn `UserConstructionScript`
  (`parent.UserConstructionScript`))