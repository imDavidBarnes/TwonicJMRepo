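; BP_FireAttack is an enemy fire projectile attack that builds on a parent Blueprint for its behavior.
; Begin play, tick, overlap and construction all pass straight through to the parent.
; Its only addition is in Explode, which runs the parent explosion and then destroys the actor after a short delay.
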(event `self.ReceiveBeginPlay`
  (`parent.ReceiveBeginPlay`))

(event `self.Explode`
  (`parent.Explode`)
  (`KismetSystemLibrary.Delay` 0.5)
  (`self.K2_DestroyActor`))

(event `self.ReceiveActorBeginOverlap`
  (params (OtherActor :type "Actor Object Reference"))
  (`parent.ReceiveActorBeginOverlap` OtherActor))

(event `self.ReceiveTick`
  (params (DeltaSeconds :type "Float (single-precision)"))
  (`parent.ReceiveTick` DeltaSeconds))

(fn `UserConstructionScript`
  (`parent.UserConstructionScript`))