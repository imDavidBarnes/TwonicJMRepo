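; Wave spawner that spawns enemies at its own location, starting on BeginPlay and advancing to the next wave when all are gone.
; Each wave's map entry gives a difficulty and per-type counts; FindEnemy resolves each enum name to a class through a data table.
; Tick prunes invalid actors from the alive list to trigger the next wave.
; Only BP_Snake receives the difficulty, and reaching the last wave has no completion logic.
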(event `self.ReceiveBeginPlay`
  (`self.StartWaveSpawn`))

(event `self.ReceiveTick`
  (params (DeltaSeconds :type "Float (single-precision)"))
  (bind _returnvalue (`BlueprintMapLibrary.Map_Length` (`self.Waves`)))
  ;[1 1 1] Check current wave and starts new wave - drew
  (for _array_element (`self.EnemiesAlive`)
    (if (not (`KismetSystemLibrary.IsValid` _array_element))
      (`KismetArrayLibrary.Array_RemoveItem` (`self.EnemiesAlive`) _array_element)
      (bind _output_get (set `self.CurrentEnemiesAlive` (`KismetMathLibrary.Clamp` (- (`self.CurrentEnemiesAlive`) 1) 0 999)))
      (if (<= (`self.CurrentEnemiesAlive`) 0)
        (set `self.CurrentWave` (`KismetMathLibrary.Clamp` (+ (`self.CurrentWave`) 1) 0 _returnvalue))
        (if (== _returnvalue (`self.CurrentWave`))
          (`/Engine/EditorBlueprintResources/StandardMacros.DoOnce` false
            (:`Completed`
              _)))
        (`self.StartWaveSpawn`)))))

(event `StartWaveSpawn`
  (bind _value (`BlueprintMapLibrary.Map_Find` (`self.Waves`) (`self.CurrentWave`)))
  ;[1 1 1] Checks wave content and spawns the right enemy and amount - drew
  (`|ExecutionSequence`
    (:`then_0`
      (for _array_element (`self.EnemyNamesCheck`)
        (set `self.Difficulty` (`.Difficulty_41_DF399F414EFCB824949FA8AC50BB6A8E` (break `/Game/Blueprints/WaveSpawner/WaveStruct` _value)) :!label _label)
        (for _ (range 1 (+ (`BlueprintMapLibrary.Map_Find` (break `/Game/Blueprints/WaveSpawner/WaveStruct` _value) _array_element) 1))
          (`self.Find Enemy` _array_element)))
      (goto _label))
    (:`then_1`
      (`KismetSystemLibrary.Delay` 1.0)
      (`KismetSystemLibrary.Delay` 2.0)
      (for _array_element_2 (`self.EnemiesAlive`)
        _))))

(fn `Find Enemy`
  (params (Enemy :type "/Game/Blueprints/WaveSpawner/WaveEnum Enum" :default "NewEnumerator6"))
  (bind _output_get (set `self.Row Name` (`|GetEnumeratorNameAsString` Enemy)))
  (bind _returnvalue (`|GetDataTableRow` "/Game/Blueprints/WaveSpawner/WaveDataTable2.WaveDataTable2" (`KismetStringLibrary.Conv_StringToName` _output_get))
    (:`then`
      (bind _returnvalue_2 (`|SpawnActorFromClass` (break `/Game/Blueprints/WaveSpawner/WaveStruct_2` _returnvalue) (`KismetMathLibrary.Conv_VectorToTransform` (`self.K2_GetActorLocation` self)) "AdjustIfPossibleButAlwaysSpawn" "OverrideRootScale" null null))
      (if (== (break `/Game/Blueprints/WaveSpawner/WaveStruct_2` _returnvalue) "/Game/Blueprints/EnemyAI/BP_Snake.BP_Snake_C")
        (bind _asbp_snake (cast `/Game/Blueprints/EnemyAI/BP_Snake` _returnvalue_2))
        (set `/Game/Blueprints/EnemyAI/BP_Snake.DifficultySnake` (`self.Difficulty`) _asbp_snake)
        (`/Game/Blueprints/EnemyAI/BP_Snake.ChangeDifficultyWaveSpawner` _asbp_snake))
      (`KismetArrayLibrary.Array_Append` (`self.EnemiesAlive`) (`|MakeArray` _returnvalue_2))
      (set `self.CurrentEnemiesAlive` (`KismetArrayLibrary.Array_Length` (`self.EnemiesAlive`))))))

(fn `UserConstructionScript`)