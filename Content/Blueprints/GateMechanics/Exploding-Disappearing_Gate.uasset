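; Gate actor that disappears when the player steps on its pressure plate.
; The first BP_Player overlap of PressureArea starts two one-shot delayed actions: ExplodingPlate snaps to EndPosition, then GateAppearance is destroyed shortly after.
; The construction script takes EndPosition from the Movement component's world location.
; StartPosition is saved at BeginPlay but unused, and PressurePadMovement repeats the EndPosition assignment without being called.
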(event `self.ReceiveBeginPlay`
  ;[1 1 1] Beginning Location
  (set `self.Start Position` (`self.K2_GetActorLocation`)))

(event `self.Pressure Area.OnComponentBeginOverlap`
  (params (OverlappedComponent :type "PrimitiveComponent Object Reference") (OtherActor :type "Actor Object Reference") (OtherComp :type "PrimitiveComponent Object Reference") (OtherBodyIndex :type Integer) (bFromSweep :type Boolean) (SweepResult :type "HitResult Structure (by ref)"))
  ;[1 1 1] Collision - Trigger
  (cast `/Game/Blueprints/Character/BP_Player` OtherActor)
  ;[1 1 1] Conditions
  (`|ExecutionSequence`
    (:`then_0`
      (`/Engine/EditorBlueprintResources/StandardMacros.DoOnce` false
        (:`Completed`
          ;[1 1 1] Pressure Pad Movement
          (`KismetSystemLibrary.Delay` 0.3)
          (`SceneComponent.K2_SetWorldLocation` (`self.Exploding Plate`) (`self.End Position`) false false))))
    (:`then_1`
      (`/Engine/EditorBlueprintResources/StandardMacros.DoOnce` false
        (:`Completed`
          ;[1 1 1] Gate Removal
          (`KismetSystemLibrary.Delay` 1.5)
          (`ActorComponent.K2_DestroyComponent` (`self.Gate Appearance`)))))))

(fn `Pressure Pad Movement`
  (set `self.End Position` (`SceneComponent.K2_GetComponentLocation` (`self.Movement`))))

(fn `UserConstructionScript`
  ;[1 1 1] End Location - Pressure Plate
  (set `self.End Position` (`SceneComponent.K2_GetComponentLocation` (`self.Movement`))))