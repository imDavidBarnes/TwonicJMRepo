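; Rotating pillar puzzle actor with three cylinders that each turn through four quarter-turn positions toward a target combination.
; RotatePillar plays a timeline that incrementally spins the selected pillar, then advances its wrapping position index and snaps it to the matching yaw.
; CheckPillarCombo then compares the positions against CorrectSequence and sets AllTrue, which blocks further rotation; nothing is wired after the solved DoOnce.
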(event `self.ReceiveBeginPlay`
  (set `self.Pillars` (`|MakeArray` (`self.Cylinder`) (`self.Cylinder1`) (`self.Cylinder2`))))

(event `RotatePillar`
  (params (SelectedPillarToMove :type Integer))
  (bind _currentpillarpos (`self.CurrentPillarPos`))
  (bind _selectedpillar (`self.SelectedPillar`))
  (bind _output (`|GetArrayItem` (`self.Pillars`) (`self.SelectedPillar`)))
  (bind _output_2 (`|GetArrayItem` (`self.Pillars`) (`self.SelectedPillar`)))
  (bind (_returnvalue_roll _returnvalue_pitch _returnvalue_yaw) (`KismetMathLibrary.BreakRotator` (`SceneComponent.K2_GetComponentRotation` _output_2)))
  (if (not (`self.AllTrue?`))
    (set `self.SelectedPillar` SelectedPillarToMove)
    (bind (_direction _newtrack_0) (`Timeline|Timeline_0` :!via `PlayFromStart`)
      (:`Update`
        (`SceneComponent.K2_SetRelativeRotation` _output_2 (`KismetMathLibrary.RLerp` (`KismetMathLibrary.MakeRotator` 0.0 0.0 _returnvalue_yaw) (`KismetMathLibrary.MakeRotator` 0.0 0.0 (+ _returnvalue_yaw 7.0)) _newtrack_0) false false))
      (:`Finished`
        (bind _result (`/Engine/EditorBlueprintResources/StandardMacros.IncrementInt` (`|GetArrayItem` _currentpillarpos _selectedpillar))
          (:`  `
            (if (>= _result 4)
              (`KismetArrayLibrary.Array_Set` _currentpillarpos _selectedpillar))
            (switch `int` (`|GetArrayItem` (`self.CurrentPillarPos`) (`self.SelectedPillar`))
              (:`0`
                (`SceneComponent.K2_SetWorldRotation` _output (`KismetMathLibrary.MakeRotator` 0.0) false false))
              (:`1`
                (`SceneComponent.K2_SetWorldRotation` _output (`KismetMathLibrary.MakeRotator` 0.0 0.0 90.0) false false))
              (:`2`
                (`SceneComponent.K2_SetWorldRotation` _output (`KismetMathLibrary.MakeRotator` 0.0 0.0 180.0) false false))
              (:`3`
                (`SceneComponent.K2_SetWorldRotation` _output (`KismetMathLibrary.MakeRotator` 0.0 0.0 270.0) false false)))
            (`self.CheckPillarCombo`)))))))

(event `CheckPillarCombo`
  (bind _pilarcheck (`self.PilarCheck`))
  (for (_array_element _array_index) (`self.CurrentPillarPos`)
    (`KismetArrayLibrary.Array_Set` (`self.PilarCheck`) _array_index (== (`|GetArrayItem` (`self.Correct Sequence`) _array_index) _array_element))
    (bind _output_get (set `self.AllTrue?` (and (`|GetArrayItem` _pilarcheck) (`|GetArrayItem` _pilarcheck 1) (`|GetArrayItem` _pilarcheck 2))))
    (if _output_get
      (`/Engine/EditorBlueprintResources/StandardMacros.DoOnce` false))))

(fn `UserConstructionScript`)