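; Merchant actor that opens a shop UI on the player's first approach and offers randomly generated pickups.
; Overlap boxes enable its input, and Exit closes the UI and restores player control.
; The first Interact spawns bomb, sword or shield pickups with random costs and bomb or weapon variants.
; A timeline then lerps them from the merchant to four display points cached at BeginPlay.
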(event `self.Box.OnComponentBeginOverlap`
  (params (OverlappedComponent :type "PrimitiveComponent Object Reference") (OtherActor :type "Actor Object Reference") (OtherComp :type "PrimitiveComponent Object Reference") (OtherBodyIndex :type Integer) (bFromSweep :type Boolean) (SweepResult :type "HitResult Structure (by ref)"))
  (bind _returnvalue (`GameplayStatics.GetPlayerController` 0))
  (bind _returnvalue_2 (`GameplayStatics.GetPlayerController` 0))
  ;[1 1 1] Opens shop when nearby - Kieran Ganner
  (if (== OtherActor "/Game/Blueprints/Character/BP_Player.BP_Player")
    (`/Engine/EditorBlueprintResources/StandardMacros.DoOnce` false
      (:`Completed`
        (`self.DisableInput` (`GameplayStatics.GetPlayerCharacter` 0) _returnvalue)
        (set `PlayerController.bShowMouseCursor` true _returnvalue)
        (cast `/Game/Blueprints/Character/BP_Player` OtherActor)
        (`self.EnableInput` _returnvalue_2)
        (bind _asplayer_hud (cast `/Game/Blueprints/UI/PlayerHUD` (`PlayerController.GetHUD` _returnvalue_2)))
        (`/Game/Blueprints/UI/PlayerHUD.Add UI` _asplayer_hud (`/Game/Blueprints/UI/PlayerHUD.MerchantNearUI` _asplayer_hud))))))

(event `self.Box.OnComponentEndOverlap`
  (params (OverlappedComponent :type "PrimitiveComponent Object Reference") (OtherActor :type "Actor Object Reference") (OtherComp :type "PrimitiveComponent Object Reference") (OtherBodyIndex :type Integer))
  ;[1 1 1] Stops merchant from reading input when too far away - Kieran Ganner
  (cast `/Game/Blueprints/Character/BP_Player` OtherActor)
  (`self.DisableInput` (`GameplayStatics.GetPlayerController` 0)))

(event `InputAction|Exit`
  (params (Key :type "Key Structure"))
  (bind _returnvalue (`GameplayStatics.GetPlayerController` 0))
  ;[1 1 1] Closes shop on exit - Kieran Ganner
  (:`Pressed`
    (`self.EnableInput` (`GameplayStatics.GetPlayerCharacter` 0) _returnvalue)
    (bind _asplayer_hud (cast `/Game/Blueprints/UI/PlayerHUD` (`PlayerController.GetHUD` _returnvalue)))
    (`/Game/Blueprints/UI/PlayerHUD.RemoveUI` _asplayer_hud (`/Game/Blueprints/UI/PlayerHUD.MerchantNearUI` _asplayer_hud))
    (set `PlayerController.bShowMouseCursor` false _returnvalue)))

(event `self.ItemBox.OnComponentBeginOverlap`
  (params (OverlappedComponent :type "PrimitiveComponent Object Reference") (OtherActor :type "Actor Object Reference") (OtherComp :type "PrimitiveComponent Object Reference") (OtherBodyIndex :type Integer) (bFromSweep :type Boolean) (SweepResult :type "HitResult Structure (by ref)"))
  ;[1 1 1] Merchant Input - Patrick Devine
  (cast `/Game/Blueprints/Character/BP_Player` OtherActor)
  (`self.EnableInput` (`GameplayStatics.GetPlayerController` 0)))

(event `self.ItemBox.OnComponentEndOverlap`
  (params (OverlappedComponent :type "PrimitiveComponent Object Reference") (OtherActor :type "Actor Object Reference") (OtherComp :type "PrimitiveComponent Object Reference") (OtherBodyIndex :type Integer))
  ;[1 1 1] Merchant Input - Patrick Devine
  (cast `/Game/Blueprints/Character/BP_Player` OtherActor)
  (`self.DisableInput` (`GameplayStatics.GetPlayerController` 0)))

(event `self.ReceiveTick`
  (params (DeltaSeconds :type "Float (single-precision)"))
  ;[1 1 1] Move Items - Patrick Devine
  (set `self.DeltaTime` DeltaSeconds))

(event `self.ReceiveBeginPlay`
  (bind _itemsendloc (`self.itemsEndLoc`))
  ;[1 1 1] Set Item locations - Patrick Devine
  (`KismetArrayLibrary.Array_Set` _itemsendloc 0 (`SceneComponent.K2_GetComponentLocation` (`self.Item0`)))
  (`KismetArrayLibrary.Array_Set` _itemsendloc 1 (`SceneComponent.K2_GetComponentLocation` (`self.Item1`)))
  (`KismetArrayLibrary.Array_Set` _itemsendloc 2 (`SceneComponent.K2_GetComponentLocation` (`self.Item2`)))
  (`KismetArrayLibrary.Array_Set` _itemsendloc 3 (`SceneComponent.K2_GetComponentLocation` (`self.Item3`))))

(event `InputAction|Interact`
  (params (Key :type "Key Structure"))
  ;[1 1 1] Move Items - Patrick Devine
  (:`Pressed`
    (`/Engine/EditorBlueprintResources/StandardMacros.DoOnce` false
      (:`Completed`
        (`self.Spawn Items`)
        (for (_array_element _array_index) (`self.itemsObject`)
          (`KismetArrayLibrary.Array_Set` (`self.itemsStartingLoc`) _array_index (`self.K2_GetActorLocation` _array_element) true))
        (bind (_direction _time) (`Timeline|MoveItems` :!via `PlayFromStart`)
          (:`Update`
            (for (_array_element_2 _array_index_2) (`self.itemsObject`)
              (`self.K2_SetActorLocation` _array_element_2 (`KismetMathLibrary.VLerp` (`|GetArrayItem` (`self.itemsStartingLoc`) _array_index_2) (`|GetArrayItem` (`self.itemsEndLoc`) _array_index_2) _time) false false))))))))

(event `Spawn Items`
  ;[1 1 1] Spawn items - Patrick Devine
  (`KismetArrayLibrary.Array_Clear` (`self.itemsObject`))
  (`self.PopulateItemsArray`)
  (for (_array_element _array_index) (`self.itemsClass`)
    (if (`KismetSystemLibrary.IsValidClass` _array_element)
      (bind _returnvalue (`|SpawnActorFromClass` _array_element (`self.GetTransform`) "AdjustIfPossibleButAlwaysSpawn" "OverrideRootScale" null null))
      (bind _asbp_interact_pickup (cast `/Game/Blueprints/Interactables/Pickups/BP_InteractPickup` _returnvalue))
      (set `/Game/Blueprints/Interactables/Pickups/BP_InteractPickup.Cost` (`KismetMathLibrary.RandomIntegerInRange` 5 10) _asbp_interact_pickup)
      (`KismetArrayLibrary.Array_Set` (`self.itemsObject`) _array_index _returnvalue true)
      (`|ExecutionSequence`
        (:`then_0`
          (bind _asbomb_pickup (cast `/Game/Blueprints/Interactables/Pickups/Bombs/BombPickup` _returnvalue))
          (switch `int` (`KismetMathLibrary.RandomIntegerInRange` 0 3)
            (:`0`
              (set `/Game/Blueprints/Interactables/Pickups/Bombs/BombPickup.BombType` "NewEnumerator0" _asbomb_pickup)
              (bind _output_get (set `/Game/Blueprints/Interactables/Pickups/Bombs/BombPickup.BombTypeText` "Explosive" _asbomb_pickup))
              (set `Pickup.name` (`KismetStringLibrary.Concat_StrStr` _output_get "Bomb") _asbomb_pickup))
            (:`1`
              (set `/Game/Blueprints/Interactables/Pickups/Bombs/BombPickup.BombType` "NewEnumerator3" _asbomb_pickup)
              (bind _output_get_2 (set `/Game/Blueprints/Interactables/Pickups/Bombs/BombPickup.BombTypeText` "Poison" _asbomb_pickup))
              (set `Pickup.name` (`KismetStringLibrary.Concat_StrStr` _output_get_2 "Bomb") _asbomb_pickup))
            (:`2`
              (set `/Game/Blueprints/Interactables/Pickups/Bombs/BombPickup.BombType` "NewEnumerator2" _asbomb_pickup)
              (bind _output_get_3 (set `/Game/Blueprints/Interactables/Pickups/Bombs/BombPickup.BombTypeText` "Fire" _asbomb_pickup))
              (set `Pickup.name` (`KismetStringLibrary.Concat_StrStr` _output_get_3 "Bomb") _asbomb_pickup))
            (:`3`
              (set `/Game/Blueprints/Interactables/Pickups/Bombs/BombPickup.BombType` "NewEnumerator1" _asbomb_pickup)
              (bind _output_get_4 (set `/Game/Blueprints/Interactables/Pickups/Bombs/BombPickup.BombTypeText` "Ice" _asbomb_pickup))
              (set `Pickup.name` (`KismetStringLibrary.Concat_StrStr` _output_get_4 "Bomb") _asbomb_pickup))))
        (:`then_1`
          (bind _asbp_sword_pickup (cast `/Game/Blueprints/Interactables/Pickups/BP_SwordPickup` _returnvalue))
          (if (== (`KismetMathLibrary.RandomInteger` 2) 0)
            (set `/Game/Blueprints/Interactables/Pickups/BP_SwordPickup.WeaponClass` "/Game/Blueprints/EquipItems/BP_Kopesh.BP_Kopesh_C" _asbp_sword_pickup)
            (bind _mesh (`Pickup.Mesh` _asbp_sword_pickup))
            (`StaticMeshComponent.SetStaticMesh` _mesh "/Game/Meshes/Weapons/Khopesh_retopo.Khopesh_retopo")
            (else
              (set `/Game/Blueprints/Interactables/Pickups/BP_SwordPickup.WeaponClass` "/Game/Blueprints/EquipItems/BP_ShepherdsCrook.BP_ShepherdsCrook_C" _asbp_sword_pickup)
              (`StaticMeshComponent.SetStaticMesh` _mesh "/Game/Meshes/Weapons/Stick_retopo.Stick_retopo"))))))))

(event `PopulateItemsArray`
  ;[1 1 1] Spawn items - Patrick Devine
  (for _index (range 4)
    (switch `int` (`KismetMathLibrary.RandomInteger` 4)
      (:`0`
        (`KismetArrayLibrary.Array_Set` (`self.itemsClass`) _index "/Game/Blueprints/Interactables/Pickups/Bombs/BombPickup.BombPickup_C"))
      (:`1`
        (`KismetArrayLibrary.Array_Set` (`self.itemsClass`) _index "/Game/Blueprints/Interactables/Pickups/Bombs/BombPickup.BombPickup_C"))
      (:`2`
        (`KismetArrayLibrary.Array_Set` (`self.itemsClass`) _index "/Game/Blueprints/Interactables/Pickups/BP_SwordPickup.BP_SwordPickup_C"))
      (:`3`
        (`KismetArrayLibrary.Array_Set` (`self.itemsClass`) _index "/Game/Blueprints/Interactables/Pickups/BP_ShieldPickup.BP_ShieldPickup_C")))))

(fn `UserConstructionScript`)