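; BP_Vase is a breakable overworld pot that drops coins when broken.
; A random drop count is rolled at BeginPlay; BreakObject spawns that many scaled-down BP_Coin actors, each worth one, then destroys the vase.
; Coins spawn at a Z offset above the vase with yaw spread evenly around a full circle.
; The construction script picks one of four pot meshes from VaseType.
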(event `self.BreakObject`
  ;[1 1 1] Vase break - Patrick Devine
  (`self.SpawnMoney`)
  (`self.K2_DestroyActor`))

(event `self.ReceiveBeginPlay`
  ;[1 1 1] Vase break - Patrick Devine
  (set `self.MoneyDropAmount` (`KismetMathLibrary.RandomIntegerInRange` 3 7)))

(event `SpawnMoney`
  (bind (_returnvalue_x _returnvalue_y _returnvalue_z) (`KismetMathLibrary.BreakVector` (`self.K2_GetActorLocation`)))
  ;[1 1 1] Vase break - Patrick Devine
  (for _index (range (`self.MoneyDropAmount`))
    (bind _returnvalue (`|SpawnActorFromClass` "/Game/Blueprints/Interactables/Pickups/BP_Coin.BP_Coin_C" (`KismetMathLibrary.MakeTransform` (`KismetMathLibrary.MakeVector` _returnvalue_x _returnvalue_y (+ _returnvalue_z (`self.ZPosOffset`))) (`KismetMathLibrary.MakeRotator` 0.0 0.0 (* _index (/ 360.0 (`KismetMathLibrary.Conv_IntToDouble` (`self.MoneyDropAmount`))))) (0.25 0.25 0.25)) "AdjustIfPossibleButAlwaysSpawn" "OverrideRootScale" null null))
    (set `Pickup.quantity` 1 _returnvalue)))

(fn `UserConstructionScript`
  (bind _staticmeshcomponent (`self.StaticMeshComponent`))
  ;[1 0.3177 0.3177] VaseType Changing - Mark Thompson
  (switch `/Game/Blueprints/OverworldObjects/E_Vases` (`self.VaseType`)
    (:`NewEnumerator0`
      (`StaticMeshComponent.SetStaticMesh` _staticmeshcomponent "/Game/Meshes/Assets/Pot_A.Pot_A"))
    (:`NewEnumerator1`
      (`StaticMeshComponent.SetStaticMesh` _staticmeshcomponent "/Game/Meshes/Assets/Pot_D.Pot_D"))
    (:`NewEnumerator2`
      (`StaticMeshComponent.SetStaticMesh` _staticmeshcomponent "/Game/Meshes/Assets/Pot_C.Pot_C"))
    (:`NewEnumerator3`
      (`StaticMeshComponent.SetStaticMesh` _staticmeshcomponent "/Game/Meshes/Assets/Pot_B.Pot_B"))))