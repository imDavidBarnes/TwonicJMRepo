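; BP_CandleRoom is a candle prop for the overworld with selectable single, dual or trio variants.
; The construction script picks the static mesh from CandleType.
; BeginPlay halves the Candlelight timeline's play rate, and that timeline's update maps its track to point light intensity for a flicker or pulse.
; No wired call starts the timeline in this graph.
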(event `self.ReceiveBeginPlay`
  (`TimelineComponent.SetPlayRate` (`self.Candlelight`) 0.5))

(fn `UserConstructionScript`
  (bind _staticmesh (`self.StaticMesh`))
  (switch `/Game/Blueprints/OverworldObjects/E_CandleTypes` (`self.Candle Type`)
    (:`NewEnumerator0`
      (`StaticMeshComponent.SetStaticMesh` _staticmesh "/Game/Meshes/Assets/Candle_Type3.Candle_Type3"))
    (:`NewEnumerator1`
      (`StaticMeshComponent.SetStaticMesh` _staticmesh "/Game/Meshes/Assets/Candle_Type2.Candle_Type2"))
    (:`NewEnumerator2`
      (`StaticMeshComponent.SetStaticMesh` _staticmesh "/Game/Meshes/Assets/Candle_Type1.Candle_Type1"))))