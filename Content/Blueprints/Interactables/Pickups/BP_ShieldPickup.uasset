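; Shield pickup that equips a shield on the player and then removes itself from the world.
; Its Pickup event stores ShieldClass on the BP_Player pawn and has SocketWeapon place it at the left hand socket.
; Begin and end overlap events only forward to the parent class.
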(event `self.ReceiveActorEndOverlap`
  (params (OtherActor :type "Actor Object Reference"))
  (`parent.ReceiveActorEndOverlap` OtherActor))

(event `self.Pickup`
  ;[1 1 1] Pickup Shield - Patrick Devine
  (bind _asbp_player (cast `/Game/Blueprints/Character/BP_Player` (`GameplayStatics.GetPlayerPawn` 0)))
  (bind _output_get (set `PlayerCharacter.BPShield` (`self.ShieldClass`) _asbp_player))
  (bind _asbp_shield (castclass `/Game/Blueprints/EquipItems/BP_Shield` _output_get))
  (`/Game/Blueprints/Character/BP_Player.SocketWeapon` _asbp_player _asbp_shield "LeftHandSocket")
  (`self.K2_DestroyActor`))

(event `self.ReceiveActorBeginOverlap`
  (params (OtherActor :type "Actor Object Reference"))
  (`parent.ReceiveActorBeginOverlap` OtherActor))

(fn `UserConstructionScript`
  (`parent.UserConstructionScript`))