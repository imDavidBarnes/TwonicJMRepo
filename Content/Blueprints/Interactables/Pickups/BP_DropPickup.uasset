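; Pickup that shoots out of an entity when spawned, following a timeline-driven path along its forward vector with a vertical component.
; On BeginPlay it disables the proximity sphere, then lerps from its start position using the Move curve, DropDistance and delta-time scaling.
; When the timeline finishes it re-enables the sphere's collision and sets GoToPlayer, though no homing logic appears in this graph.
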(event `self.ReceiveBeginPlay`
  (bind _startpos (`self.StartPos`))
  (bind _returnvalue (/ (`self.DropDistance`) (`self.DeltaTime`)))
  (bind (_returnvalue_x _returnvalue_y) (`KismetMathLibrary.BreakVector` (* (`self.GetActorForwardVector`) _returnvalue)))
  ;[1 1 1] Shoot drop out of entity - Patrick Devine
  (set `self.StartPos` (`self.K2_GetActorLocation`))
  (set `self.GoToPlayer` false)
  (`PrimitiveComponent.SetCollisionEnabled` (`self.ProxSphere`) "NoCollision")
  (bind (_direction _move) (`Timeline|MoveDropOutwards` :!via `PlayFromStart`)
    (:`Update`
      (`self.K2_SetActorRelativeLocation` (`KismetMathLibrary.VLerp` _startpos (+ (`/Game/Blueprints/BP_MacroLib.DeltaTime` (`self.DeltaTime`) (* _move (`KismetMathLibrary.MakeVector` _returnvalue_x _returnvalue_y _returnvalue))) _startpos) (`TimelineComponent.GetPlaybackPosition` (`self.MoveDropOutwards`)))))
    (:`Finished`
      (`PrimitiveComponent.SetCollisionEnabled` (`self.ProxSphere`) "QueryAndPhysics")
      (set `self.GoToPlayer` true))))

(fn `UserConstructionScript`
  (`parent.UserConstructionScript`))