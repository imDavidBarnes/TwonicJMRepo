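; BP_SwordPickup is a weapon pickup that gives the player either a Khopesh or a Shepherd's Crook, based on its WeaponClass.
; BeginPlay sets the static mesh to match that class.
; Pickup assigns the class to BP_Player, attaches it through SocketWeapon with a weapon-specific socket, saves both in BP_GameInstance, then destroys the pickup.
; Overlap and Tick events only forward to the parent.
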(event `self.ReceiveBeginPlay`
  (bind _weaponclass (`self.WeaponClass`))
  (bind _mesh (`self.Mesh`))
  (`|ExecutionSequence`
    (:`then_1`
      (`parent.ReceiveBeginPlay`)
      (if (== _weaponclass "/Game/Blueprints/EquipItems/BP_Kopesh.BP_Kopesh_C")
        (`StaticMeshComponent.SetStaticMesh` _mesh "/Game/Meshes/Weapons/Khopesh_retopo.Khopesh_retopo")
        (elif (== _weaponclass "/Game/Blueprints/EquipItems/BP_ShepherdsCrook.BP_ShepherdsCrook_C")
          (`StaticMeshComponent.SetStaticMesh` _mesh "/Game/Meshes/Weapons/Stick_retopo.Stick_retopo"))))))

(event `self.ReceiveActorEndOverlap`
  (params (OtherActor :type "Actor Object Reference"))
  (`parent.ReceiveActorEndOverlap` OtherActor))

(event `self.ReceiveActorBeginOverlap`
  (params (OtherActor :type "Actor Object Reference"))
  (`parent.ReceiveActorBeginOverlap` OtherActor))

(event `self.Pickup`
  (bind _socket_name_crook (`self.Socket Name Crook`))
  (bind _socket_name_kopesh (`self.Socket Name kopesh`))
  (bind _weaponclass (`self.WeaponClass`))
  ;[1 1 1] Pickup Sword - Patrick Devine
  (bind _asbp_player (cast `/Game/Blueprints/Character/BP_Player` (`GameplayStatics.GetPlayerPawn` 0)))
  (set `PlayerCharacter.BPWeapon` (`self.WeaponClass`) _asbp_player)
  (if (== _weaponclass "/Game/Blueprints/EquipItems/BP_Kopesh.BP_Kopesh_C")
    (bind _asbp_kopesh (castclass `/Game/Blueprints/EquipItems/BP_Kopesh` (`self.WeaponClass`)))
    (set `self.name` "Khopesh")
    (`/Game/Blueprints/Character/BP_Player.SocketWeapon` _asbp_player _asbp_kopesh _socket_name_kopesh)
    (bind _asbp_game_instance (cast `/Game/Blueprints/BP_GameInstance` (`GameplayStatics.GetGameInstance`)))
    (`/Game/Blueprints/BP_GameInstance.SaveCurrentWeapon` _asbp_game_instance (`self.WeaponClass`) _socket_name_kopesh)
    (`self.K2_DestroyActor`)
    (elif (== _weaponclass "/Game/Blueprints/EquipItems/BP_ShepherdsCrook.BP_ShepherdsCrook_C")
      (bind _asbp_shepherds_crook (castclass `/Game/Blueprints/EquipItems/BP_ShepherdsCrook` (`self.WeaponClass`)))
      (set `self.name` "Shepherds Crook")
      (`/Game/Blueprints/Character/BP_Player.SocketWeapon` _asbp_player _asbp_shepherds_crook _socket_name_crook)
      (bind _asbp_game_instance_2 (cast `/Game/Blueprints/BP_GameInstance` (`GameplayStatics.GetGameInstance`)))
      (`/Game/Blueprints/BP_GameInstance.SaveCurrentWeapon` _asbp_game_instance_2 (`self.WeaponClass`) _socket_name_crook)
      (`self.K2_DestroyActor`))))

(event `self.ReceiveTick`
  (params (DeltaSeconds :type "Float (single-precision)"))
  (`parent.ReceiveTick` DeltaSeconds))

(fn `UserConstructionScript`
  (`parent.UserConstructionScript`))