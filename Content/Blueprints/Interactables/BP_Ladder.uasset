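; Interactable ladder that lets the player climb up or down between its bottom and top.
; Overlap triggers at each end show a prompt widget and enable Interact input when the ladder is available and unused.
; Interacting snaps the player on and sets BP_Player's Climbing flag while timelines reposition them, zeroing velocity, until a height threshold places them at the other end.
; The construction script positions LadderTop from LadderHeight.
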(event `InputAction|Interact`
  (params (Key :type "Key Structure"))
  (bind _returnvalue (`GameplayStatics.GetPlayerCharacter` 0))
  (bind _returnvalue_2 (`GameplayStatics.GetPlayerCharacter` 0))
  (bind _returnvalue_3 (`SceneComponent.K2_GetComponentToWorld` (`self.Top_Off`)))
  (bind (_returnvalue_location _returnvalue_rotation) (`KismetMathLibrary.BreakTransform` (`SceneComponent.K2_GetComponentToWorld` (`self.Bottom_On`))))
  (bind (_returnvalue_x _returnvalue_y) (`KismetMathLibrary.BreakVector` (`SceneComponent.K2_GetComponentLocation` (`Character.Mesh` _returnvalue))))
  ;[0.269 1 0.6006] Conrad Dakarn
  ;;[1 1 1] Checks that Character is at bottom of ladder and sets it in use
  (:`Pressed`
    (if (`self.Bottom_Interact`)
      (set `self.In_Use` true)
      ;;[1 1 1] Sets Character facing bottom of ladder
      (`SceneComponent.K2_SetWorldTransform` (`Actor.RootComponent` _returnvalue_2) (`KismetMathLibrary.MakeTransform` _returnvalue_location _returnvalue_rotation) false false)
      ;;[1 1 1] Sets character velocity to zero - Stops character flying off randomly after "teleport"
      (set `MovementComponent.Velocity` (0.0 0.0 0.0) (`Character.CharacterMovement` _returnvalue_2))
      ;;[1 1 1] Plays Animation To Climb - Drew
      (bind _asbp_player (cast `/Game/Blueprints/Character/BP_Player` (`GameplayStatics.GetPlayerCharacter` 0)))
      (set `/Game/Blueprints/Character/BP_Player.Climbing` true _asbp_player)
      (bind (_direction _newtrack_1) (`Timeline|ClimbUP` :!via `PlayFromStart` :!label _label)
        (:`Update`
          (if (>= (.z _newtrack_1) (`self.ladder_height`))
            ;[1 1 1] Teleports The Player To Top Of Ladder - Drew
            (`SceneComponent.K2_SetWorldTransform` (`Actor.RootComponent` (`GameplayStatics.GetPlayerCharacter` 0)) (`KismetMathLibrary.MakeTransform` (`KismetMathLibrary.MakeVector` (.x (.location _returnvalue_3)) (.y (.location _returnvalue_3)) (.z (.location _returnvalue_3))) (.rotation _returnvalue_3)) false false)
            (set `self.In_Use` false)
            (bind _asbp_player_2 (cast `/Game/Blueprints/Character/BP_Player` (`GameplayStatics.GetPlayerCharacter` 0)))
            (set `/Game/Blueprints/Character/BP_Player.Climbing` false _asbp_player_2)
            (goto _label :!via `Stop`)
            (else
              ;;[1 1 1] Moves Character to top of ladder facing away from it
              (`SceneComponent.K2_SetWorldTransform` (`Actor.RootComponent` _returnvalue) (`KismetMathLibrary.MakeTransform` (`KismetMathLibrary.MakeVector` _returnvalue_x _returnvalue_y (+ (.z _newtrack_1) (.z (.location (`SceneComponent.K2_GetComponentToWorld` (`self.Bottom_On`)))))) (.rotation (`SceneComponent.K2_GetComponentToWorld` (`self.Top_Off`)))) false false)
              ;;[1 1 1] Sets character velocity to zero - Stops character flying off randomly after "teleport"
              (set `MovementComponent.Velocity` (0.0 0.0 0.0) (`Character.CharacterMovement` _returnvalue))
              ;;[1 1 1] Allows bottom to be interacted with and disables "in use" status
              (set `self.Bottom_Interact` true))))))))

(event `self.ladder_bottom.OnComponentBeginOverlap`
  (params (OverlappedComponent :type "PrimitiveComponent Object Reference") (OtherActor :type "Actor Object Reference") (OtherComp :type "PrimitiveComponent Object Reference") (OtherBodyIndex :type Integer) (bFromSweep :type Boolean) (SweepResult :type "HitResult Structure (by ref)"))
  ;[0.269 1 0.6006] Conrad Dakarn
  (if (== OtherActor (`GameplayStatics.GetPlayerCharacter` 0))
    (if (`self.Available`)
      (if (not (`self.In_Use`))
        (`SceneComponent.SetVisibility` (`self.ClimbUpLadderWidget`) true false)
        (set `self.Bottom_Interact` true)
        (set `self.Top_Interact` false)
        (`self.EnableInput` (`GameplayStatics.GetPlayerController` 0))))))

(event `self.ladder_bottom.OnComponentEndOverlap`
  (params (OverlappedComponent :type "PrimitiveComponent Object Reference") (OtherActor :type "Actor Object Reference") (OtherComp :type "PrimitiveComponent Object Reference") (OtherBodyIndex :type Integer))
  ;[0.269 1 0.6006] Conrad Dakarn
  (if (== OtherActor (`GameplayStatics.GetPlayerCharacter` 0))
    (`SceneComponent.SetVisibility` (`self.ClimbUpLadderWidget`) false false)
    (`self.DisableInput` (`GameplayStatics.GetPlayerController` 0))))

(event `InputAction|Interact`
  (params (Key :type "Key Structure"))
  (bind _returnvalue (`GameplayStatics.GetPlayerCharacter` 0))
  (bind _returnvalue_2 (`GameplayStatics.GetPlayerCharacter` 0))
  (bind (_returnvalue_location _returnvalue_rotation) (`KismetMathLibrary.BreakTransform` (`SceneComponent.K2_GetComponentToWorld` (`self.Top_On`))))
  (bind _returnvalue_3 (`SceneComponent.K2_GetComponentToWorld` (`self.Bottom_On`)))
  (bind _returnvalue_4 (`SceneComponent.K2_GetComponentToWorld` (`self.Bottom_On`)))
  ;[0.269 1 0.6006] Conrad Dakarn
  ;;[1 1 1] Checks that Character is at top of ladder and sets it in use
  (:`Pressed`
    (if (`self.Top_Interact`)
      (set `self.In_Use` true)
      ;;[1 1 1] Sets Character facing top of ladder
      (`SceneComponent.K2_SetWorldTransform` (`Actor.RootComponent` _returnvalue) (`KismetMathLibrary.MakeTransform` _returnvalue_location _returnvalue_rotation) false false)
      ;;[1 1 1] Sets character velocity to zero - Stops character flying off randomly after "teleport"
      (set `MovementComponent.Velocity` (0.0 0.0 0.0) (`Character.CharacterMovement` _returnvalue))
      ;;[1 1 1] Plays Animation To Climb - Drew
      (bind _asbp_player (cast `/Game/Blueprints/Character/BP_Player` (`GameplayStatics.GetPlayerCharacter` 0)))
      (set `/Game/Blueprints/Character/BP_Player.Climbing` true _asbp_player)
      (bind (_direction _newtrack_1) (`Timeline|Timeline_1` :!via `PlayFromStart` :!label _label_2)
        (:`Update`
          (if (<= (.z _newtrack_1) (`self.Ladder_HeightDown`))
            ;[1 1 1] Teleports The Player To Top Of Ladder - Drew
            (`SceneComponent.K2_SetWorldTransform` (`Actor.RootComponent` (`GameplayStatics.GetPlayerCharacter` 0)) (`KismetMathLibrary.MakeTransform` (`KismetMathLibrary.MakeVector` (.x (.location _returnvalue_4)) (.y (.location _returnvalue_4)) (+ (.z (.location _returnvalue_4)) 100.0)) (.rotation _returnvalue_4)) false false)
            (set `self.In_Use` false)
            (bind _asbp_player_2 (cast `/Game/Blueprints/Character/BP_Player` (`GameplayStatics.GetPlayerCharacter` 0)))
            (set `/Game/Blueprints/Character/BP_Player.Climbing` false _asbp_player_2)
            (goto _label_2 :!via `Stop`)
            (else
              ;;[1 1 1] Moves Character to top of ladder facing away from it
              (`SceneComponent.K2_SetWorldTransform` (`Actor.RootComponent` _returnvalue_2) (`KismetMathLibrary.MakeTransform` (`KismetMathLibrary.MakeVector` (.x (.location _returnvalue_3)) (.y (.location _returnvalue_3)) (+ (.z (.location (`SceneComponent.K2_GetComponentToWorld` (`self.Top_On`)))) (.z _newtrack_1))) (.rotation _returnvalue_3)) false false)
              ;;[1 1 1] Sets character velocity to zero - Stops character flying off randomly after "teleport"
              (set `MovementComponent.Velocity` (0.0 0.0 0.0) (`Character.CharacterMovement` _returnvalue_2))
              ;;[1 1 1] Allows top to be interacted with and disables "in use" status
              (set `self.Top_Interact` true))))))))

(event `self.ladder_top.OnComponentBeginOverlap`
  (params (OverlappedComponent :type "PrimitiveComponent Object Reference") (OtherActor :type "Actor Object Reference") (OtherComp :type "PrimitiveComponent Object Reference") (OtherBodyIndex :type Integer) (bFromSweep :type Boolean) (SweepResult :type "HitResult Structure (by ref)"))
  ;[0.269 1 0.6006] Conrad Dakarn
  (if (== OtherActor (`GameplayStatics.GetPlayerCharacter` 0))
    (if (`self.Available`)
      (if (not (`self.In_Use`))
        (`SceneComponent.SetVisibility` (`self.ClimbDownLadderWidget`) true false)
        (set `self.Bottom_Interact` false)
        (set `self.Top_Interact` true)
        (`self.EnableInput` (`GameplayStatics.GetPlayerController` 0))))))

(event `self.ladder_top.OnComponentEndOverlap`
  (params (OverlappedComponent :type "PrimitiveComponent Object Reference") (OtherActor :type "Actor Object Reference") (OtherComp :type "PrimitiveComponent Object Reference") (OtherBodyIndex :type Integer))
  ;[0.269 1 0.6006] Conrad Dakarn
  (if (== OtherActor (`GameplayStatics.GetPlayerCharacter` 0))
    (`SceneComponent.SetVisibility` (`self.ClimbDownLadderWidget`) false false)
    (`self.DisableInput` (`GameplayStatics.GetPlayerController` 0))))

(event `self.ReceiveBeginPlay`
  (set `self.Ladder_HeightDown` (+ (- (`self.Ladder_HeightDown`) (`self.ladder_height`)) 100.0)))

(fn `UserConstructionScript`
  (`SceneComponent.K2_SetRelativeLocation` (`self.ladder_top`) (`KismetMathLibrary.MakeVector` 200.0 0.0 (`self.ladder_height`)) false false))