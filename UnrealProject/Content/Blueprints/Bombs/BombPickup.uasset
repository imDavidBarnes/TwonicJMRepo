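; Bomb pickup actor that adds one bomb of its configured type to the player's count, then destroys itself.
; A sphere overlap with BP_Player sets InRange, shows a prompt widget and enables input on the actor; leaving reverses all three.
; Pressing Interact while in range compares the BombType enum, converted to a string at BeginPlay, against each type name to call the matching per-type increment function.
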(event `self.ReceiveBeginPlay`
  ;[1 1 1] Bomb Select - Drew
  (set `self.BombTypeText` (`|GetEnumeratorNameAsString` (`self.BombType`))))

(event `InputAction|Interact`
  (params (Key :type "Key Structure"))
  ;[1 1 1] Bomb Select - Drew
  (:`Pressed`
    (`self.PickupBomb`)))

(event `PickupBomb`
  ;[1 1 1] Bomb Select - Drew
  (if (`self.InRange?`)
    (`|ExecutionSequence`
      (:`then_0`
        (if (`KismetStringLibrary.EqualEqual_StrStr` (`self.BombTypeText`) "ExplosiveBomb")
          (`self.ExplosiveBomb`)))
      (:`then_1`
        (if (`KismetStringLibrary.EqualEqual_StrStr` (`self.BombTypeText`) "IceBomb")
          (`self.IceBomb`)))
      (:`then_2`
        (if (`KismetStringLibrary.EqualEqual_StrStr` (`self.BombTypeText`) "FireBomb")
          (`self.FireBomb`)))
      (:`then_3`
        (if (`KismetStringLibrary.EqualEqual_StrStr` (`self.BombTypeText`) "PoisonBomb")
          (`self.PoisonBomb`))))))

(event `self.Sphere1.OnComponentBeginOverlap`
  (params (OverlappedComponent :type "PrimitiveComponent Object Reference") (OtherActor :type "Actor Object Reference") (OtherComp :type "PrimitiveComponent Object Reference") (OtherBodyIndex :type Integer) (bFromSweep :type Boolean) (SweepResult :type "HitResult Structure (by ref)"))
  ;[1 1 1] Bomb Select - Drew
  (cast `/Game/Blueprints/Character/BP_Player` OtherActor)
  (set `self.InRange?` true)
  (`SceneComponent.SetVisibility` (`self.Widget`) true false)
  (`self.EnableInput` (`GameplayStatics.GetPlayerController` 0)))

(event `self.Sphere1.OnComponentEndOverlap`
  (params (OverlappedComponent :type "PrimitiveComponent Object Reference") (OtherActor :type "Actor Object Reference") (OtherComp :type "PrimitiveComponent Object Reference") (OtherBodyIndex :type Integer))
  ;[1 1 1] Bomb Select - Drew
  (cast `/Game/Blueprints/Character/BP_Player` OtherActor)
  (set `self.InRange?` false)
  (`SceneComponent.SetVisibility` (`self.Widget`) false false)
  (`self.DisableInput` (`GameplayStatics.GetPlayerController` 0)))

(fn `ExplosiveBomb`
  (bind _asbp_player (cast `/Game/Blueprints/Character/BP_Player` (`GameplayStatics.GetPlayerCharacter` 0)))
  (set `/Game/Blueprints/Character/BP_Player.ExplosiveBombAmount` (+ (`/Game/Blueprints/Character/BP_Player.ExplosiveBombAmount` _asbp_player) 1) _asbp_player)
  (`self.K2_DestroyActor`))

(fn `FireBomb`
  (bind _asbp_player (cast `/Game/Blueprints/Character/BP_Player` (`GameplayStatics.GetPlayerCharacter` 0)))
  (bind _output_get (set `/Game/Blueprints/Character/BP_Player.FireBombAmount` (+ (stale _output_get) 1) _asbp_player))
  (`self.K2_DestroyActor`))

(fn `IceBomb`
  (bind _asbp_player (cast `/Game/Blueprints/Character/BP_Player` (`GameplayStatics.GetPlayerCharacter` 0)))
  (bind _output_get (set `/Game/Blueprints/Character/BP_Player.IceBombAmount` (+ (stale _output_get) 1) _asbp_player))
  (`self.K2_DestroyActor`))

(fn `PoisonBomb`
  (bind _asbp_player (cast `/Game/Blueprints/Character/BP_Player` (`GameplayStatics.GetPlayerCharacter` 0)))
  (bind _output_get (set `/Game/Blueprints/Character/BP_Player.PoisonBombAmount` (+ (stale _output_get) 1) _asbp_player))
  (`self.K2_DestroyActor`))

(fn `UserConstructionScript`)