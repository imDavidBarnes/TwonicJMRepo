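; PoisonBomb is a projectile bomb that explodes on first contact with a MainEnemyPawn or three seconds after spawning.
; Detonation activates a radial force, enables the initially disabled Explosion collision, adds a Niagara effect, stops movement, removes the projectile component and schedules cleanup.
; Explosion overlap calls ExplosionDamage behind a DoOnce, so only the first enemy caught is damaged; a player damage branch is left disconnected.
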(event `self.EnemyCollision.OnComponentBeginOverlap`
  (params (OverlappedComponent :type "PrimitiveComponent Object Reference") (OtherActor :type "Actor Object Reference") (OtherComp :type "PrimitiveComponent Object Reference") (OtherBodyIndex :type Integer) (bFromSweep :type Boolean) (SweepResult :type "HitResult Structure (by ref)"))
  ;[1 1 1] Checks if hit enemy - Drew
  (cast `/Game/Blueprints/EnemyAI/MainEnemyPawn` OtherActor)
  (`/Engine/EditorBlueprintResources/StandardMacros.DoOnce` false
    (:`Completed`
      (set `self.HitAlready?` true)
      ;[1 1 1] Activates Explosion and collisions - Drew
      (`ActorComponent.Activate` (`self.RadialForce`) false :!label _label)
      (`PrimitiveComponent.SetCollisionEnabled` (`self.Explosion`) "QueryAndPhysics")
      (`AddComponent|NODE_AddNiagaraComponent-0`)
      (`MovementComponent.StopMovementImmediately` (`self.ProjectileMovement`))
      (`/Engine/EditorBlueprintResources/StandardMacros.IsValid` (`self.ExplosiveProjectile`)
        (:`Is Valid`
          (`ActorComponent.K2_DestroyComponent` (`self.ExplosiveProjectile`))
          (`|ExecutionSequence`
            (:`then_0`
              (`KismetSystemLibrary.Delay` 3.0)
              (`self.K2_DestroyActor`))
            (:`then_1`
              (`KismetSystemLibrary.Delay` 1.0)
              (`ActorComponent.Deactivate` (`self.RadialForce`)))))))))

(event `self.ReceiveBeginPlay`
  ;[1 1 1] Activates Explosion and collisions - Drew
  (`PrimitiveComponent.SetCollisionEnabled` (`self.Explosion`) "NoCollision")
  (`KismetSystemLibrary.Delay` 3.0)
  (if (not (`self.HitAlready?`))
    (goto _label)))

(event `self.Explosion.OnComponentBeginOverlap`
  (params (OverlappedComponent :type "PrimitiveComponent Object Reference") (OtherActor :type "Actor Object Reference") (OtherComp :type "PrimitiveComponent Object Reference") (OtherBodyIndex :type Integer) (bFromSweep :type Boolean) (SweepResult :type "HitResult Structure (by ref)"))
  ;[1 1 1] Runs Events to damage the enemy when hit with explosion - Drew
  (`|ExecutionSequence`
    (:`then_1`
      (bind _asmain_enemy_pawn (cast `/Game/Blueprints/EnemyAI/MainEnemyPawn` OtherActor))
      (`/Engine/EditorBlueprintResources/StandardMacros.DoOnce` false
        (:`Completed`
          (`/Game/Blueprints/EnemyAI/MainEnemyPawn.ExplosionDamage` _asmain_enemy_pawn))))))

(fn `UserConstructionScript`)