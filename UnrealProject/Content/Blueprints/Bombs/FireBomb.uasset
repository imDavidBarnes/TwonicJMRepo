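; Fire bomb projectile that bursts into a burning area when it overlaps an enemy pawn or after a three-second fuse.
; Ignition stops movement, enables the Fire collision and adds a Niagara effect, then destroys the actor after a delay.
; Enemy overlaps with Fire set a timer whose looping follows OnFire, but its FireDMG event is empty.
; A player explosive-damage branch is disconnected.
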(event `self.EnemyCollision.OnComponentBeginOverlap`
  (params (OverlappedComponent :type "PrimitiveComponent Object Reference") (OtherActor :type "Actor Object Reference") (OtherComp :type "PrimitiveComponent Object Reference") (OtherBodyIndex :type Integer) (bFromSweep :type Boolean) (SweepResult :type "HitResult Structure (by ref)"))
  ;[1 1 1] Checks if hit enemy - Drew
  (cast `/Game/Blueprints/EnemyAI/MainEnemyPawn` OtherActor)
  (`/Engine/EditorBlueprintResources/StandardMacros.DoOnce` false
    (:`Completed`
      (set `self.HitAlready?` true)
      ;[1 1 1] Activates Explosion and collisions - Drew
      (`PrimitiveComponent.SetCollisionEnabled` (`self.Fire`) "QueryAndPhysics" :!label _label)
      (`AddComponent|NODE_AddNiagaraComponent-1`)
      (`MovementComponent.StopMovementImmediately` (`self.ProjectileMovement`))
      (`/Engine/EditorBlueprintResources/StandardMacros.IsValid` (`self.FireProjectile`)
        (:`Is Valid`
          (`KismetSystemLibrary.Delay` 5.0)
          (`self.K2_DestroyActor`))))))

(event `self.ReceiveBeginPlay`
  ;[1 1 1] Activates Explosion and collisions - Drew
  (`PrimitiveComponent.SetCollisionEnabled` (`self.Fire`) "NoCollision")
  (`KismetSystemLibrary.Delay` 3.0)
  (if (`self.HitAlready?`)
    (`PrimitiveComponent.SetCollisionEnabled` (`self.Fire`) "QueryAndPhysics")
    (else
      (goto _label))))

(event `self.Fire.OnComponentBeginOverlap`
  (params (OverlappedComponent :type "PrimitiveComponent Object Reference") (OtherActor :type "Actor Object Reference") (OtherComp :type "PrimitiveComponent Object Reference") (OtherBodyIndex :type Integer) (bFromSweep :type Boolean) (SweepResult :type "HitResult Structure (by ref)"))
  ;[1 1 1] Runs Events to damage the enemy when hit with explosion - Drew
  (cast `/Game/Blueprints/EnemyAI/MainEnemyPawn` OtherActor)
  (bind _output_get (set `self.OnFire` true))
  (`KismetSystemLibrary.K2_SetTimerDelegate` (delegate `FireDMG`) 1.5 _output_get :!label _label_2))

(event `self.Fire.OnComponentEndOverlap`
  (params (OverlappedComponent :type "PrimitiveComponent Object Reference") (OtherActor :type "Actor Object Reference") (OtherComp :type "PrimitiveComponent Object Reference") (OtherBodyIndex :type Integer))
  ;[1 1 1] Runs Events to damage the enemy when hit with explosion - Drew
  (cast `/Game/Blueprints/EnemyAI/MainEnemyPawn` OtherActor)
  (set `self.OnFire` false)
  (goto _label_2))

(event `FireDMG`
  ;[1 1 1] Runs Events to damage the enemy when hit with explosion - Drew
)

(fn `UserConstructionScript`)