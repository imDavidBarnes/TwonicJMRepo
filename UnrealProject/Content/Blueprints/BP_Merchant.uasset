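; BP_Merchant is a merchant actor that lets the player open and close a shop UI.
; A box overlap with BP_Player enables or disables the merchant's own input, so Interact and Exit only respond near it.
; Interact disables player input and swaps PlayerHUD's player UI for the merchant UI.
; Exit restores player input and swaps the UIs back.
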(event `self.Box.OnComponentBeginOverlap`
  (params (OverlappedComponent :type "PrimitiveComponent Object Reference") (OtherActor :type "Actor Object Reference") (OtherComp :type "PrimitiveComponent Object Reference") (OtherBodyIndex :type Integer) (bFromSweep :type Boolean) (SweepResult :type "HitResult Structure (by ref)"))
  ;[1 1 1] Enables/Disables input when overlapped - Kieran Ganner
  (cast `/Game/Blueprints/Character/BP_Player` OtherActor)
  (`self.EnableInput` (`GameplayStatics.GetPlayerController` 0)))

(event `self.Box.OnComponentEndOverlap`
  (params (OverlappedComponent :type "PrimitiveComponent Object Reference") (OtherActor :type "Actor Object Reference") (OtherComp :type "PrimitiveComponent Object Reference") (OtherBodyIndex :type Integer))
  ;[1 1 1] Enables/Disables input when overlapped - Kieran Ganner
  (cast `/Game/Blueprints/Character/BP_Player` OtherActor)
  (`self.DisableInput` (`GameplayStatics.GetPlayerController` 0)))

(event `InputAction|Interact`
  (params (Key :type "Key Structure"))
  ;[1 1 1] Opens shop when interacted with - Kieran Ganner
  (:`Pressed`
    (bind _asplayer_hud (cast `/Game/Blueprints/UI/PlayerHUD` (`PlayerController.GetHUD` (`GameplayStatics.GetPlayerController` 0))))
    (`/Game/Blueprints/UI/PlayerHUD.RemoveUI` _asplayer_hud (`/Game/Blueprints/UI/PlayerHUD.PlayerUI` _asplayer_hud))
    (bind _asbp_player (cast `/Game/Blueprints/Character/BP_Player` (`GameplayStatics.GetPlayerCharacter` 0)))
    (`self.DisableInput` _asbp_player (`GameplayStatics.GetPlayerController` 0))
    (`/Game/Blueprints/UI/PlayerHUD.Add UI` _asplayer_hud (`/Game/Blueprints/UI/PlayerHUD.MerchantUI` _asplayer_hud))))

(event `InputAction|Exit`
  (params (Key :type "Key Structure"))
  (bind _returnvalue (`GameplayStatics.GetPlayerController` 0))
  ;[1 1 1] Closes shop when exited - Kieran Ganner
  (:`Pressed`
    (bind _asbp_player (cast `/Game/Blueprints/Character/BP_Player` (`GameplayStatics.GetPlayerCharacter` 0)))
    (`self.EnableInput` _asbp_player _returnvalue)
    (bind _asplayer_hud (cast `/Game/Blueprints/UI/PlayerHUD` (`PlayerController.GetHUD` _returnvalue)))
    (`/Game/Blueprints/UI/PlayerHUD.Add UI` _asplayer_hud (`/Game/Blueprints/UI/PlayerHUD.PlayerUI` _asplayer_hud))
    (`/Game/Blueprints/UI/PlayerHUD.RemoveUI` _asplayer_hud (`/Game/Blueprints/UI/PlayerHUD.MerchantUI` _asplayer_hud))))

(fn `UserConstructionScript`)