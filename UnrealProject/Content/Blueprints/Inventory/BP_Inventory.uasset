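; Inventory actor that stores pickups in an Items map and freezes gameplay while the inventory is showing.
; Tick checks IsShowing to disable player and enemy movement, block attack, block and roll, and show the cursor.
; When hidden, a DoOnce restores walking, input flags and cursor, re-arming only inside the enemy loop while showing.
; AddItem and RemoveItem edit the map and print debug results.
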(event `TurnOnPlayerInput`
  ;[1 1 1] Make sure player can't dodge or attack - Patrick Devine
  (bind _asbp_player (cast `/Game/Blueprints/Character/BP_Player` (`GameplayStatics.GetPlayerPawn` 0)))
  (set `/Game/Blueprints/Character/BP_Player.CanAttack` true _asbp_player)
  (set `/Game/Blueprints/Character/BP_Player.CanBlock` true _asbp_player)
  (set `/Game/Blueprints/Character/BP_Player.CanRoll` true _asbp_player))

(event `TurnOffPlayerInput`
  ;[1 1 1] Make sure player can't dodge or attack - Patrick Devine
  (bind _asbp_player (cast `/Game/Blueprints/Character/BP_Player` (`GameplayStatics.GetPlayerPawn` 0)))
  (set `/Game/Blueprints/Character/BP_Player.CanAttack` false _asbp_player)
  (set `/Game/Blueprints/Character/BP_Player.CanBlock` false _asbp_player)
  (set `/Game/Blueprints/Character/BP_Player.CanRoll` false _asbp_player))

(event `self.ReceiveTick`
  (params (DeltaSeconds :type "Float (single-precision)"))
  (bind _returnvalue (`GameplayStatics.GetPlayerController` 0))
  (bind _charactermovement (`Character.CharacterMovement` (`GameplayStatics.GetPlayerCharacter` 0)))
  ;[1 1 1] Inven HUD
  (if (`self.isShowing`)
    (`self.TurnOffPlayerInput`)
    (`CharacterMovementComponent.DisableMovement` _charactermovement)
    (set `PlayerController.bShowMouseCursor` true _returnvalue)
    (bind _outactors (`GameplayStatics.GetAllActorsOfClass` "/Game/Blueprints/EnemyAI/MainEnemyPawn.MainEnemyPawn_C"))
    (for _array_element _outactors
      (`CharacterMovementComponent.DisableMovement` (`Character.CharacterMovement` _array_element))
      (`self.Reset movement set`))
    (else
      (`/Engine/EditorBlueprintResources/StandardMacros.DoOnce` false :!label _label
        (:`Completed`
          (`CharacterMovementComponent.SetMovementMode` _charactermovement "MOVE_Walking" 0)
          (set `PlayerController.bShowMouseCursor` false _returnvalue)
          (bind _outactors_2 (`GameplayStatics.GetAllActorsOfClass` "/Game/Blueprints/EnemyAI/MainEnemyPawn.MainEnemyPawn_C"))
          (for _array_element_2 _outactors_2
            (`CharacterMovementComponent.SetMovementMode` (`Character.CharacterMovement` _array_element_2) "MOVE_Walking" 0)
            (`self.TurnOnPlayerInput`)))))))

(event `Reset movement set`
  ;[1 1 1] Inven HUD
  (goto _label :!via `Reset`))

(fn `AddItem`
  (params (pickup :type "Pickup Class Reference") (AddItem :type Name))
  (bind _items (`self.items`))
  (`BlueprintMapLibrary.Map_Add` _items AddItem pickup)
  (if (`.ReturnValue` (`BlueprintMapLibrary.Map_Find` _items AddItem))
    (`KismetSystemLibrary.PrintString` (`KismetStringLibrary.Concat_StrStr` (`KismetStringLibrary.Conv_NameToString` AddItem) " was added to inven") true true (struct :`R` 0.337497 :`G` 1.0 :`B` 0.411363 :`A` 1.0))
    (else
      (`KismetSystemLibrary.PrintString` "failed to add" true true (struct :`R` 1.0 :`G` 0.266788 :`B` 0.217016 :`A` 1.0)))))

(fn `RemoveItem`
  (params (pickup :type Name))
  (bind _items (`self.items`))
  (if (`.ReturnValue` (`BlueprintMapLibrary.Map_Find` _items pickup))
    (bind _returnvalue (`BlueprintMapLibrary.Map_Remove` _items pickup))
    (if _returnvalue
      (`KismetSystemLibrary.PrintString` (`KismetStringLibrary.Concat_StrStr` (`KismetStringLibrary.Conv_NameToString` pickup) " was removed") true true (struct :`R` 0.337497 :`G` 1.0 :`B` 0.411363 :`A` 1.0))
      (else
        (`KismetSystemLibrary.PrintString` "failed to remove" true true (struct :`R` 1.0 :`G` 0.266788 :`B` 0.217016 :`A` 1.0))))
    (else
      (`KismetSystemLibrary.PrintString` "item not found"))))

(fn `UserConstructionScript`)