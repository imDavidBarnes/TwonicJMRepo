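; BP_Kopesh is an equip-item Blueprint for the Kopesh weapon that removes itself when it is no longer the player's weapon.
; Every Tick it casts the first player pawn to BP_Player and destroys itself if BPWeapon does not match BP_Kopesh.
; BeginPlay, overlap and construction only call the parent, and Tick also runs the parent logic before its check.
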(event `self.ReceiveBeginPlay`
  (`parent.ReceiveBeginPlay`))

(event `self.ReceiveActorBeginOverlap`
  (params (OtherActor :type "Actor Object Reference"))
  (`parent.ReceiveActorBeginOverlap` OtherActor))

(event `self.ReceiveTick`
  (params (DeltaSeconds :type "Float (single-precision)"))
  (`parent.ReceiveTick` DeltaSeconds)
  (bind _asbp_player (cast `/Game/Blueprints/Character/BP_Player` (`GameplayStatics.GetPlayerPawn` 0)))
  (if (!= (`PlayerCharacter.BPWeapon` _asbp_player) "BP_Kopesh_C")
    (`self.K2_DestroyActor`)))

(fn `UserConstructionScript`
  (`parent.UserConstructionScript`))