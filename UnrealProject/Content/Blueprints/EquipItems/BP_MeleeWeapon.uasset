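; Melee weapon Blueprint that supports charging attack damage and knockback over time.
; IncrementDamage and IncrementKnockback each raise their value by a rate scaled with world delta seconds, clamped to a maximum.
; IsFullyCharged reports when both values reach their caps, and ReturnToNormal resets them to base damage and minimum knockback.
; The event graph is empty, so nothing in this Blueprint calls these functions.
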(fn `IncrementDamage`
  (set `self.AttackDamage` (`KismetMathLibrary.FMin` (`self.MaxDamage`) (+ (`self.AttackDamage`) (* (`self.ROI_Damage`) (`GameplayStatics.GetWorldDeltaSeconds`))))))

(fn `IncrementKnockback`
  (set `self.KnockbackPercent` (`KismetMathLibrary.FMin` (+ (`self.KnockbackPercent`) (* (`GameplayStatics.GetWorldDeltaSeconds`) (`self.ROI_KnockbackPercent`))) (`self.MaxKnockbackPercent`))))

(fn `IsFullyCharged`
  (returns (IsCharged :type Boolean))
  (if (and (== (`self.KnockbackPercent`) (`self.MaxKnockbackPercent`)) (== (`self.AttackDamage`) (`self.MaxDamage`)))
    (return true)
    (else
      (return false))))

(fn `ReturnToNormal`
  (set `self.KnockbackPercent` (`self.MinKnockbackPercent`))
  (set `self.AttackDamage` (`self.BaseDamage`)))

(fn `UserConstructionScript`)