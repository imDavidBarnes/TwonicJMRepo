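; Weapon pickup that equips the player with either a Kopesh or a Shepherd's Crook, based on its WeaponClass.
; BeginPlay picks the matching display mesh, sword or great hammer, while overlap and tick defer to the parent.
; Pickup sets the player's weapon, attaches it to that weapon's socket, saves class and socket to the game instance, then destroys itself.
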(event `self.ReceiveBeginPlay`
  (bind _mesh (`self.Mesh`))
  (bind _weaponclass (`self.WeaponClass`))
  (`|ExecutionSequence`
    (:`then_1`
      (`parent.ReceiveBeginPlay`)
      (if (== _weaponclass "/Game/Blueprints/EquipItems/BP_Kopesh.BP_Kopesh_C")
        (`StaticMeshComponent.SetStaticMesh` _mesh "/Game/Weapon_Pack/Mesh/Weapons/Weapons_Kit/SM_Sword.SM_Sword")
        (elif (== _weaponclass "/Game/Blueprints/EquipItems/BP_ShepherdsCrook.BP_ShepherdsCrook_C")
          (`StaticMeshComponent.SetStaticMesh` _mesh "/Game/Weapon_Pack/Mesh/Weapons/Weapons_Kit/SM_GreatHammer.SM_GreatHammer"))))))

(event `self.ReceiveActorEndOverlap`
  (params (OtherActor :type "Actor Object Reference"))
  (`parent.ReceiveActorEndOverlap` OtherActor))

(event `self.ReceiveActorBeginOverlap`
  (params (OtherActor :type "Actor Object Reference"))
  (`parent.ReceiveActorBeginOverlap` OtherActor))

(event `self.Pickup`
  (bind _socket_name_crook (`self.Socket Name Crook`))
  (bind _socket_name_kopesh (`self.Socket Name kopesh`))
  (bind _weaponclass (`self.WeaponClass`))
  ;[1 1 1] Pickup Sword - Patrick Devine
  (bind _asbp_player (cast `/Game/Blueprints/Character/BP_Player` (`GameplayStatics.GetPlayerPawn` 0)))
  (set `PlayerCharacter.BPWeapon` (`self.WeaponClass`) _asbp_player)
  (if (== _weaponclass "/Game/Blueprints/EquipItems/BP_Kopesh.BP_Kopesh_C")
    (bind _asbp_kopesh (castclass `/Game/Blueprints/EquipItems/BP_Kopesh` (`self.WeaponClass`)))
    (`/Game/Blueprints/Character/BP_Player.SocketWeapon` _asbp_player _asbp_kopesh _socket_name_kopesh)
    (bind _asbp_game_instance (cast `/Game/Blueprints/BP_GameInstance` (`GameplayStatics.GetGameInstance`)))
    (`/Game/Blueprints/BP_GameInstance.SaveCurrentWeapon` _asbp_game_instance (`self.WeaponClass`) _socket_name_kopesh)
    (`self.K2_DestroyActor`)
    (elif (== _weaponclass "/Game/Blueprints/EquipItems/BP_ShepherdsCrook.BP_ShepherdsCrook_C")
      (bind _asbp_shepherds_crook (castclass `/Game/Blueprints/EquipItems/BP_ShepherdsCrook` (`self.WeaponClass`)))
      (`/Game/Blueprints/Character/BP_Player.SocketWeapon` _asbp_player _asbp_shepherds_crook _socket_name_crook)
      (bind _asbp_game_instance_2 (cast `/Game/Blueprints/BP_GameInstance` (`GameplayStatics.GetGameInstance`)))
      (`/Game/Blueprints/BP_GameInstance.SaveCurrentWeapon` _asbp_game_instance_2 (`self.WeaponClass`) _socket_name_crook)
      (`self.K2_DestroyActor`)
      (else
        (`KismetSystemLibrary.PrintString` "Weapon Class null")))))

(event `self.ReceiveTick`
  (params (DeltaSeconds :type "Float (single-precision)"))
  (`parent.ReceiveTick` DeltaSeconds))

(fn `UserConstructionScript`
  (`parent.UserConstructionScript`))