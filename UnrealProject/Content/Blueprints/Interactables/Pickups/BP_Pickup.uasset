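; BP_Pickup is a pickup actor that spins in place and can be drawn toward the player.
; Each tick it yaws by RotSpeed and, if GoToPlayer is enabled, gets the vector to BP_Player from ToPlayer.
; Within RangeOfCollection, it moves along that normalized direction at SpeedOfCollection, scaled by delta time, without sweeping.
; The graph contains no collection or overlap logic.
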(event `self.ReceiveTick`
  (params (DeltaSeconds :type "Float (single-precision)"))
  ;[1 1 1] Move pickups towards player when enabled - Patrick Devine
  (set `self.DeltaTime` DeltaSeconds)
  (`self.K2_AddActorLocalRotation` (`KismetMathLibrary.MakeRotator` 0.0 0.0 (* (`self.RotSpeed`) (`self.DeltaTime`))))
  (if (`self.GoToPlayer`)
    (bind _toplayer (`self.ToPlayer`))
    (if (<= (`KismetMathLibrary.VSize` _toplayer) (`self.RangeOfCollection`))
      (`self.K2_SetActorLocation` (+ (* (`/Game/Blueprints/BP_MacroLib.DeltaTime` (`self.DeltaTime`) (`KismetMathLibrary.Normal` _toplayer)) (`self.SpeedOfCollection`)) (`self.K2_GetActorLocation`))))))

(fn `ToPlayer`
  (returns (ToPlayer :type "Vector Structure"))
  (bind _asbp_player (cast `/Game/Blueprints/Character/BP_Player` (`GameplayStatics.GetPlayerPawn` 0)))
  (return (- (`self.K2_GetActorLocation` _asbp_player) (`self.K2_GetActorLocation`))))

(fn `UserConstructionScript`)