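; Parent Blueprint for interactable pickups that the player collects, with an optional purchase cost.
; Overlapping BP_Player toggles CanPickup and enables input on the actor.
; Pressing Interact while in range deducts any positive Cost from player money, then calls the empty Pickup event and adds the item's class and name through InvenRef.
; An older AddToInventory path remains disconnected, and a BP_Inventory actor lookup goes unused.
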(event `InputAction|Interact`
  (params (Key :type "Key Structure"))
  ;[1 1 1] Old add to inven
)

(event `self.ReceiveBeginPlay`
  ;[1 1 1] Parent interact pickup - Patrick Devine
)

(event `Pickup`
  ;[1 1 1] Parent interact pickup - Patrick Devine
)

(event `self.ReceiveActorEndOverlap`
  (params (OtherActor :type "Actor Object Reference"))
  ;[1 1 1] Parent interact pickup - Patrick Devine
  (cast `/Game/Blueprints/Character/BP_Player` OtherActor)
  (set `self.CanPickup` false))

(event `self.ReceiveActorBeginOverlap`
  (params (OtherActor :type "Actor Object Reference"))
  ;[1 1 1] Parent interact pickup - Patrick Devine
  (cast `/Game/Blueprints/Character/BP_Player` OtherActor)
  (set `self.CanPickup` true)
  (`self.EnableInput` (`GameplayStatics.GetPlayerController` 0)))

(event `self.ReceiveTick`
  (params (DeltaSeconds :type "Float (single-precision)"))
  ;[1 1 1] Parent interact pickup - Patrick Devine
  (`parent.ReceiveTick` DeltaSeconds))

(event `InputAction|Interact`
  (params (Key :type "Key Structure"))
  (:`Pressed`
    (if (`self.CanPickup`)
      (bind _asbp_player (cast `/Game/Blueprints/Character/BP_Player` (`GameplayStatics.GetPlayerPawn` 0)))
      ;[0.5089 0.7084 0.305] Adding item to the inventory - mia
      (if (> (`self.Cost`) 0)
        (bind _returnvalue (`PlayerCharacter.RemoveFromMoney` _asbp_player (`self.Cost`)))
        (if _returnvalue
          (`self.Pickup` :!label _label)
          (bind _outactors (`GameplayStatics.GetAllActorsOfClass` "/Game/Blueprints/Inventory/BP_Inventory.BP_Inventory_C"))
          (`/Game/Blueprints/Inventory/BP_Inventory.AddItem` (`/Game/Blueprints/Character/BP_Player.invenRef` _asbp_player) (`self.PickupClass`) (`KismetStringLibrary.Conv_StringToName` (`self.name`))))
        (else
          (goto _label))))))

(fn `UserConstructionScript`
  (`parent.UserConstructionScript`))