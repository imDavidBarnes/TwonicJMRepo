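; Health pickup that launches itself along its forward direction when spawned, with its quantity set from the truncated healing amount.
; The MoveDrop timeline drives an incremental arc, scaling delta-time-adjusted curve values by a random distance that is re-rolled during updates.
; Proximity collision stays off during flight, then turns on as GoToPlayer is set.
; Tick and construction defer to the parent class.
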(event `self.ReceiveBeginPlay`
  ;[1 1 1] Shoot coins out in every direction - Patrick Devine
  (set `self.GoToPlayer` false)
  (`self.Send Forward`))

(event `Send Forward`
  (bind _returnvalue (`KismetMathLibrary.RandomFloatInRange` (`self.HealthDropDistance`) 500.0))
  (bind (_returnvalue_x _returnvalue_y) (`KismetMathLibrary.BreakVector` (* (`KismetMathLibrary.Normal` (`self.GetActorForwardVector`)) _returnvalue)))
  ;[1 1 1] Shoot coins out in every direction - Patrick Devine
  (`PrimitiveComponent.SetCollisionEnabled` (`self.ProxSphere`) "NoCollision")
  (set `self.quantity` (`KismetMathLibrary.FTrunc` (`self.HealingAmount`)))
  (bind (_direction _move) (`Timeline|MoveDrop` :!via `PlayFromStart`)
    (:`Update`
      (bind (_deltavector_x _deltavector_y _deltavector_z) (`KismetMathLibrary.BreakVector` (`/Game/Blueprints/BP_MacroLib.DeltaTime` (`self.DeltaTime`) (`KismetMathLibrary.MakeVector` (.x _move) (.y _move) (.z _move)))))
      (bind (_returnvalue_x_2 _returnvalue_y_2) (`KismetMathLibrary.BreakVector` (* (`KismetMathLibrary.MakeVector` _deltavector_x _deltavector_y) (`KismetMathLibrary.MakeVector` _returnvalue_x _returnvalue_y))))
      (`self.K2_SetActorLocation` (+ (`KismetMathLibrary.MakeVector` _returnvalue_x_2 _returnvalue_y_2 (* _deltavector_z _returnvalue)) (`self.K2_GetActorLocation`))))
    (:`Finished`
      (`PrimitiveComponent.SetCollisionEnabled` (`self.ProxSphere`) "QueryAndPhysics")
      (set `self.GoToPlayer` true))))

(event `self.ReceiveTick`
  (params (DeltaSeconds :type "Float (single-precision)"))
  ;[1 1 1] Shoot coins out in every direction - Patrick Devine
  (`parent.ReceiveTick` DeltaSeconds))

(fn `UserConstructionScript`
  (`parent.UserConstructionScript`))