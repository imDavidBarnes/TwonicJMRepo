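; Interactable ladder that moves the player between bottom and top by teleporting, with no actual climbing movement.
; Bottom and top overlaps enable input and set which end responds to Interact, if the ladder is available and not in use.
; Interact snaps the player to that end, waits in proportion to LadderHeight, then teleports to the far exit, zeroing velocity each time.
; The construction script positions the top from LadderHeight; debug prints stand in for interact UI.
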(event `InputAction|Interact`
  (params (Key :type "Key Structure"))
  (bind _returnvalue (`GameplayStatics.GetPlayerCharacter` 0))
  (bind _returnvalue_2 (`GameplayStatics.GetPlayerCharacter` 0))
  (bind (_returnvalue_location _returnvalue_rotation) (`KismetMathLibrary.BreakTransform` (`SceneComponent.K2_GetComponentToWorld` (`self.Bottom_On`))))
  (bind (_returnvalue_location_2 _returnvalue_rotation_2) (`KismetMathLibrary.BreakTransform` (`SceneComponent.K2_GetComponentToWorld` (`self.Top_Off`))))
  ;[0.269 1 0.6006] Conrad Dakarn
  ;;[1 1 1] Checks that Character is at bottom of ladder and sets it in use
  (:`Pressed`
    (if (`self.Bottom_Interact`)
      (`KismetSystemLibrary.PrintString` "Bottom Pressed--- PLEASE WAIT" true true (struct :`G` 0.66 :`B` 1.0 :`A` 1.0) 20.0)
      (set `self.In_Use` true)
      ;;[1 1 1] Sets Character facing bottom of ladder
      (`SceneComponent.K2_SetWorldTransform` (`Actor.RootComponent` _returnvalue_2) (`KismetMathLibrary.MakeTransform` _returnvalue_location _returnvalue_rotation) false false)
      ;;[1 1 1] Sets character velocity to zero - Stops character flying off randomly after "teleport"
      (set `MovementComponent.Velocity` (0.0 0.0 0.0) (`Character.CharacterMovement` _returnvalue_2))
      ;;[1 1 1] Pauses "teleport" based on ladder height - Allows animation to run
      (`KismetSystemLibrary.Delay` (/ (`self.ladder_height`) 200.0))
      ;;[1 1 1] Moves Character to top of ladder facing away from it
      (`SceneComponent.K2_SetWorldTransform` (`Actor.RootComponent` _returnvalue) (`KismetMathLibrary.MakeTransform` _returnvalue_location_2 _returnvalue_rotation_2) false false)
      ;;[1 1 1] Sets character velocity to zero - Stops character flying off randomly after "teleport"
      (set `MovementComponent.Velocity` (0.0 0.0 0.0) (`Character.CharacterMovement` _returnvalue))
      ;;[1 1 1] Allows bottom to be interacted with and disables "in use" status
      (set `self.Bottom_Interact` true)
      (`KismetSystemLibrary.PrintString` "Bottom On  - End of Bottom Event" true true (struct :`G` 0.66 :`B` 1.0 :`A` 1.0) 20.0)
      (set `self.In_Use` false))))

(event `self.ladder_bottom.OnComponentBeginOverlap`
  (params (OverlappedComponent :type "PrimitiveComponent Object Reference") (OtherActor :type "Actor Object Reference") (OtherComp :type "PrimitiveComponent Object Reference") (OtherBodyIndex :type Integer) (bFromSweep :type Boolean) (SweepResult :type "HitResult Structure (by ref)"))
  ;[0.269 1 0.6006] Conrad Dakarn
  (if (== OtherActor (`GameplayStatics.GetPlayerCharacter` 0))
    (if (`self.Available`)
      (if (not (`self.In_Use`))
        (`KismetSystemLibrary.PrintString` "Add Interact UI Here" true true (struct :`G` 0.66 :`B` 1.0 :`A` 1.0) 20.0)
        (set `self.Bottom_Interact` true)
        (set `self.Top_Interact` false)
        (`KismetSystemLibrary.PrintString` "Bottom On - Top Off - Bottom Overlap" true true (struct :`G` 0.66 :`B` 1.0 :`A` 1.0) 20.0)
        (`self.EnableInput` (`GameplayStatics.GetPlayerController` 0))))))

(event `self.ladder_bottom.OnComponentEndOverlap`
  (params (OverlappedComponent :type "PrimitiveComponent Object Reference") (OtherActor :type "Actor Object Reference") (OtherComp :type "PrimitiveComponent Object Reference") (OtherBodyIndex :type Integer))
  ;[0.269 1 0.6006] Conrad Dakarn
  (if (== OtherActor (`GameplayStatics.GetPlayerCharacter` 0))
    (`self.DisableInput` (`GameplayStatics.GetPlayerController` 0))))

(event `InputAction|Interact`
  (params (Key :type "Key Structure"))
  (bind _returnvalue (`GameplayStatics.GetPlayerCharacter` 0))
  (bind _returnvalue_2 (`GameplayStatics.GetPlayerCharacter` 0))
  (bind (_returnvalue_location _returnvalue_rotation) (`KismetMathLibrary.BreakTransform` (`SceneComponent.K2_GetComponentToWorld` (`self.Top_On`))))
  (bind (_returnvalue_location_2 _returnvalue_rotation_2) (`KismetMathLibrary.BreakTransform` (`SceneComponent.K2_GetComponentToWorld` (`self.Bottom_Off`))))
  ;[0.269 1 0.6006] Conrad Dakarn
  (:`Pressed`
    (if (`self.Top_Interact`)
      (`KismetSystemLibrary.PrintString` "Top Pressed" true true (struct :`R` 1.0 :`G` 0.021788 :`A` 1.0) 20.0)
      (set `self.In_Use` true)
      (`SceneComponent.K2_SetWorldTransform` (`Actor.RootComponent` _returnvalue) (`KismetMathLibrary.MakeTransform` _returnvalue_location _returnvalue_rotation) false false)
      (set `MovementComponent.Velocity` (0.0 0.0 0.0) (`Character.CharacterMovement` _returnvalue))
      (`KismetSystemLibrary.Delay` (/ (`self.ladder_height`) 200.0))
      (`SceneComponent.K2_SetWorldTransform` (`Actor.RootComponent` _returnvalue_2) (`KismetMathLibrary.MakeTransform` _returnvalue_location_2 _returnvalue_rotation_2) false false)
      (set `MovementComponent.Velocity` (0.0 0.0 0.0) (`Character.CharacterMovement` _returnvalue_2))
      (set `self.Top_Interact` true)
      (`KismetSystemLibrary.PrintString` "Top On -  End TTop Event" true true (struct :`R` 1.0 :`G` 0.0174 :`A` 1.0) 20.0)
      (set `self.In_Use` false))))

(event `self.ladder_top.OnComponentBeginOverlap`
  (params (OverlappedComponent :type "PrimitiveComponent Object Reference") (OtherActor :type "Actor Object Reference") (OtherComp :type "PrimitiveComponent Object Reference") (OtherBodyIndex :type Integer) (bFromSweep :type Boolean) (SweepResult :type "HitResult Structure (by ref)"))
  ;[0.269 1 0.6006] Conrad Dakarn
  (if (== OtherActor (`GameplayStatics.GetPlayerCharacter` 0))
    (if (`self.Available`)
      (if (not (`self.In_Use`))
        (`KismetSystemLibrary.PrintString` "Add Interact UI Here" true true (struct :`R` 1.0 :`G` 0.023403 :`A` 1.0) 20.0)
        (set `self.Bottom_Interact` false)
        (set `self.Top_Interact` true)
        (`KismetSystemLibrary.PrintString` "Bottom Off - Top On -Top Overlap" true true (struct :`R` 1.0 :`G` 0.035563 :`A` 1.0) 20.0)
        (`self.EnableInput` (`GameplayStatics.GetPlayerController` 0))))))

(event `self.ladder_top.OnComponentEndOverlap`
  (params (OverlappedComponent :type "PrimitiveComponent Object Reference") (OtherActor :type "Actor Object Reference") (OtherComp :type "PrimitiveComponent Object Reference") (OtherBodyIndex :type Integer))
  ;[0.269 1 0.6006] Conrad Dakarn
  (if (== OtherActor (`GameplayStatics.GetPlayerCharacter` 0))
    (`self.DisableInput` (`GameplayStatics.GetPlayerController` 0))))

(fn `UserConstructionScript`
  (`SceneComponent.K2_SetRelativeLocation` (`self.ladder_top`) (`KismetMathLibrary.MakeVector` 200.0 0.0 (`self.ladder_height`)) false false))