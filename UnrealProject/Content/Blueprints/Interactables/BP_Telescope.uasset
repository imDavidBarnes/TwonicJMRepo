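; Interactable telescope that, when in range, lets the player toggle a zoomed camera view offset toward the level centre flag.
; Interact flips the zoom state, then briefly disables the actor's input to block rapid toggling.
; Every Tick drives BP_Player's SetNewZoom with either max zoom and the offset to the flag, or only the speeds when not zoomed.
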(event `self.ReceiveBeginPlay`
  ;[0.1557 0.9702 1] Handle Input in BP for now - Patrick Devine
  (`self.EnableInput` (`GameplayStatics.GetPlayerController` 0)))

(event `DelayKey`
  (bind _returnvalue (`GameplayStatics.GetPlayerController` 0))
  ;[0.1557 0.9702 1] Handle Input in BP for now - Patrick Devine
  (`self.DisableInput` _returnvalue)
  (`KismetSystemLibrary.Delay` 1.0)
  (`self.EnableInput` _returnvalue))

(event `InputAction|Interact`
  (params (Key :type "Key Structure"))
  ;[0.1557 0.9702 1] Set zoom once player is in range of telescope - Patrick Devine
  (:`Pressed`
    (if (`self.InRange`)
      (set `self.ShouldZoom` (not (`self.ShouldZoom`)))
      (`self.DelayKey`))))

(event `self.ReceiveTick`
  (params (DeltaSeconds :type "Float (single-precision)"))
  (bind _returnvalue (`GameplayStatics.GetPlayerPawn` 0))
  ;[0.1557 0.9702 1] Zoom and set offset - Patrick Devine
  (if (`self.ShouldZoom`)
    (bind _asbp_player (cast `/Game/Blueprints/Character/BP_Player` _returnvalue))
    (bind _asbp_level_centre_flag (castclass `/Game/Blueprints/BP_LevelCentreFlag` (`self.LevelCentre`)))
    (bind _returnvalue_2 (`GameplayStatics.GetActorOfClass` _asbp_level_centre_flag))
    (`/Game/Blueprints/Character/BP_Player.SetNewZoom` _asbp_player (`self.MaxZoom`) (- (`self.K2_GetActorLocation` _returnvalue_2) (`self.K2_GetActorLocation` _asbp_player)) (`self.ZoomSpeed`) (`self.OffsetSpeed`))
    (else
      (bind _asbp_player_2 (cast `/Game/Blueprints/Character/BP_Player` _returnvalue))
      (`/Game/Blueprints/Character/BP_Player.SetNewZoom` _asbp_player_2 1710.0 (0.0 0.0 0.0) (`self.ZoomSpeed`) (`self.OffsetSpeed`)))))

(fn `UserConstructionScript`)