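; Merchant actor that opens a shop UI when BP_Player enters its Box trigger.
; On first overlap it disables player input, shows the cursor, takes input itself and adds MerchantNearUI through PlayerHUD.
; The Exit action restores player input and removes the UI; leaving Box disables merchant input.
; Ending overlap with ItemBox destroys all BP_TempItem actors, resetting the open-once gate for each one destroyed.
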(event `self.Box.OnComponentBeginOverlap`
  (params (OverlappedComponent :type "PrimitiveComponent Object Reference") (OtherActor :type "Actor Object Reference") (OtherComp :type "PrimitiveComponent Object Reference") (OtherBodyIndex :type Integer) (bFromSweep :type Boolean) (SweepResult :type "HitResult Structure (by ref)"))
  (bind _returnvalue (`GameplayStatics.GetPlayerController` 0))
  (bind _returnvalue_2 (`GameplayStatics.GetPlayerController` 0))
  ;[1 1 1] Opens shop when nearby - Kieran Ganner
  (if (== OtherActor "/Game/Blueprints/Character/BP_Player.BP_Player")
    (`/Engine/EditorBlueprintResources/StandardMacros.DoOnce` false :!label _label
      (:`Completed`
        (`self.DisableInput` (`GameplayStatics.GetPlayerCharacter` 0) _returnvalue)
        (set `PlayerController.bShowMouseCursor` true _returnvalue)
        (cast `/Game/Blueprints/Character/BP_Player` OtherActor)
        (`self.EnableInput` _returnvalue_2)
        (bind _asplayer_hud (cast `/Game/Blueprints/UI/PlayerHUD` (`PlayerController.GetHUD` _returnvalue_2)))
        (`/Game/Blueprints/UI/PlayerHUD.Add UI` _asplayer_hud (`/Game/Blueprints/UI/PlayerHUD.MerchantNearUI` _asplayer_hud))))))

(event `self.ItemBox.OnComponentEndOverlap`
  (params (OverlappedComponent :type "PrimitiveComponent Object Reference") (OtherActor :type "Actor Object Reference") (OtherComp :type "PrimitiveComponent Object Reference") (OtherBodyIndex :type Integer))
  ;[1 1 1] Despawns item when too far away - Kieran Ganner
  (bind _outactors (`GameplayStatics.GetAllActorsOfClass` "/Game/Blueprints/Merchant/BP_TempItem.BP_TempItem_C"))
  (for _array_element _outactors
    (`self.K2_DestroyActor` _array_element)
    (goto _label :!via `Reset`)))

(event `self.Box.OnComponentEndOverlap`
  (params (OverlappedComponent :type "PrimitiveComponent Object Reference") (OtherActor :type "Actor Object Reference") (OtherComp :type "PrimitiveComponent Object Reference") (OtherBodyIndex :type Integer))
  ;[1 1 1] Stops merchant from reading input when too far away - Kieran Ganner
  (cast `/Game/Blueprints/Character/BP_Player` OtherActor)
  (`self.DisableInput` (`GameplayStatics.GetPlayerController` 0)))

(event `InputAction|Exit`
  (params (Key :type "Key Structure"))
  (bind _returnvalue (`GameplayStatics.GetPlayerController` 0))
  ;[1 1 1] Closes shop on exit - Kieran Ganner
  (:`Pressed`
    (`self.EnableInput` (`GameplayStatics.GetPlayerCharacter` 0) _returnvalue)
    (bind _asplayer_hud (cast `/Game/Blueprints/UI/PlayerHUD` (`PlayerController.GetHUD` _returnvalue)))
    (`/Game/Blueprints/UI/PlayerHUD.RemoveUI` _asplayer_hud (`/Game/Blueprints/UI/PlayerHUD.MerchantNearUI` _asplayer_hud))
    (set `PlayerController.bShowMouseCursor` false _returnvalue)))

(fn `UserConstructionScript`)