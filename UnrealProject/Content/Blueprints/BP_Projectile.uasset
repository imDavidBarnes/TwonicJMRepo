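; BP_Projectile is a projectile actor that flies straight along its spawn facing and damages the first actor it overlaps, then destroys itself.
; The construction script caches the forward vector, nudges the actor one unit along it and disables collision.
; BeginPlay re-enables collision after a short delay, then destroys the actor five seconds later.
; Tick moves it by teleporting a Speed-scaled step each frame, without delta-time scaling.
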(event `self.ReceiveBeginPlay`
  ;[1 1 1] Destroy actor after five seconds, turn on collision after 0.2 seconds
  (`KismetSystemLibrary.Delay` 0.2)
  (`self.SetActorEnableCollision` true)
  (`KismetSystemLibrary.Delay` 5.0)
  (`self.K2_DestroyActor`))

(event `self.ReceiveTick`
  (params (DeltaSeconds :type "Float (single-precision)"))
  ;[1 1 1] Move projectile forward - Patrick & Keiran
  (`self.K2_TeleportTo` (+ (`self.K2_GetActorLocation`) (* (`self.MoveVector`) (`self.Speed`))) (`self.K2_GetActorRotation`)))

(event `self.ReceiveActorBeginOverlap`
  (params (OtherActor :type "Actor Object Reference"))
  ;[1 1 1] Event hit (on collision destroy self)
  (`GameplayStatics.ApplyDamage` OtherActor (`self.Damage`) null self)
  (`self.K2_DestroyActor`))

(fn `UserConstructionScript`
  ;[1 1 1] Spawn projectile and move to starting pos (disable collision) - Patrick & Keiran
  (bind _output_get (set `self.MoveVector` (`SceneComponent.GetForwardVector` (`self.DefaultSceneRoot`))))
  (`self.K2_TeleportTo` (+ _output_get (`self.K2_GetActorLocation`)) (`self.K2_GetActorRotation`))
  (`self.SetActorEnableCollision` false))