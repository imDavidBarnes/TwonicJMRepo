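; Bridge trigger actor that spawns piranhas while the player overlaps it.
; Begin and end overlap with BP_Player toggle a spawn flag, which Tick checks alongside a count of living BP_Piranha actors.
; When none exist, every EnemySpawner set to piranha spawns one, using the spawner's transform with Y replaced by the player's current Y to line up with them.
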(event `self.ReceiveActorBeginOverlap`
  (params (OtherActor :type "Actor Object Reference"))
  ;[1 1 1] Spawn Piranha when player is on bridge - Patrick Devine
  (bind _asbp_player (cast `/Game/Blueprints/Character/BP_Player` OtherActor))
  (set `self.SpawnFish` true)
  (bind (_returnvalue_x _returnvalue_y) (`KismetMathLibrary.BreakVector` (`self.K2_GetActorLocation` _asbp_player)))
  (set `self.PlayerY` _returnvalue_y))

(event `self.ReceiveActorEndOverlap`
  (params (OtherActor :type "Actor Object Reference"))
  ;[1 1 1] Spawn Piranha when player is on bridge - Patrick Devine
  (cast `/Game/Blueprints/Character/BP_Player` OtherActor)
  (set `self.SpawnFish` false))

(event `Spawn fish`
  ;[1 1 1] Spawn Piranha when player is on bridge - Patrick Devine
  (bind _outactors (`GameplayStatics.GetAllActorsOfClass` "/Game/Blueprints/EnemyAI/EnemySpawner.EnemySpawner_C"))
  (for _array_element _outactors
    (if (== (`/Game/Blueprints/EnemyAI/EnemySpawner.EnemyToSpawn` _array_element) "/Game/Blueprints/EnemyAI/BP_Piranha.BP_Piranha_C")
      (bind _asbp_player (cast `/Game/Blueprints/Character/BP_Player` (`GameplayStatics.GetPlayerPawn` 0)))
      (bind (_returnvalue_x _returnvalue_y) (`KismetMathLibrary.BreakVector` (`self.K2_GetActorLocation` _asbp_player)))
      (bind _output_get (set `self.PlayerY` _returnvalue_y))
      (bind _returnvalue (`self.GetTransform` _array_element))
      (`|SpawnActorFromClass` "/Game/Blueprints/EnemyAI/BP_Piranha.BP_Piranha_C" (`KismetMathLibrary.MakeTransform` (`KismetMathLibrary.MakeVector` (.x (.location _returnvalue)) _output_get (.z (.location _returnvalue))) (.rotation _returnvalue) (.scale _returnvalue)) "AdjustIfPossibleButAlwaysSpawn" "OverrideRootScale" null null))))

(event `self.ReceiveTick`
  (params (DeltaSeconds :type "Float (single-precision)"))
  ;[1 1 1] Spawn Piranha when player is on bridge - Patrick Devine
  (if (`self.SpawnFish`)
    (bind _outactors (`GameplayStatics.GetAllActorsOfClass` "/Game/Blueprints/EnemyAI/BP_Piranha.BP_Piranha_C"))
    (if (== (`KismetArrayLibrary.Array_Length` _outactors) 0)
      (`KismetSystemLibrary.Delay` 0.0)
      (`self.Spawn fish`))))

(fn `UserConstructionScript`)