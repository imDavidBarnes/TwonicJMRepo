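; Anubis boss enemy that faces the player every tick and has melee and ranged fireball attacks.
; While attacking, it chases the player with AI MoveTo until close, then calls EnemyAttack and clears the attacking state.
; Otherwise, a self-resetting DoOnce on Tick rerolls low random odds to spawn BP_FireAttack within a longer range.
; InitiateAttack starts the melee state, but its only call in this graph is disconnected.
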(event `GoToPlayer`
  ;[1 1 1] Walk to player - Patrick Devine
  (bind _asbp_player (cast `/Game/Blueprints/Character/BP_Player` (`GameplayStatics.GetPlayerPawn` 0)))
  (`|AIMoveTo` self (0.0 0.0 0.0) _asbp_player))

(event `FireProjectile`
  ;[1 1 1] Firing fire ball - Patrick Devine
  (`self.AttackSense` (* (`self.Range`) 4.0))
  (if (`self.InRange`)
    (`|SpawnActorFromClass` "/Game/Blueprints/EnemyAI/EnemyProjectileAttacks/BP_FireAttack.BP_FireAttack_C" (`KismetMathLibrary.MakeTransform` (`self.K2_GetActorLocation`) (`self.K2_GetActorRotation`) (0.5 0.5 0.5)) "AlwaysSpawn" "OverrideRootScale" self null)
    (`KismetSystemLibrary.Delay` 2.0)
    (`self.Reset Attack Rand`)
    (else
      (`self.Reset Attack Rand`))))

(event `self.ReceiveBeginPlay`
  (`parent.ReceiveBeginPlay`)
  (set `self.CanSee` true))

(event `Initiate Attack`
  ;[1 1 1] Cycling attacks on random - Patrick Devine
  (set `self.InRange` false)
  (set `self.Attacking` true))

(event `Reset Attack Rand`
  (bind _returnvalue (`KismetMathLibrary.RandomIntegerInRange` 0 100))
  ;[1 1 1] Cycling attacks on random - Patrick Devine
  (goto _label :!via `Reset`))

(event `self.ReceiveTick`
  (params (DeltaSeconds :type "Float (single-precision)"))
  (bind _returnvalue (`KismetMathLibrary.RandomIntegerInRange` 0 100))
  (set `self.DeltaTime` DeltaSeconds)
  (`self.AttackSense` (/ (`self.Range`) 3.0))
  (`self.Face Player`)
  (if (`self.Attacking`)
    (if (`self.InRange`)
      ;[1 1 1] Cycling attacks on random - Patrick Devine
      (bind _toplayer (`self.GetToPlayer`))
      (`self.EnemyAttack` _toplayer 2.5)
      (set `self.Attacking` false)
      (`|AIMoveTo` self (`self.K2_GetActorLocation`) null
        (:`OnSuccess`
          _)
        (:`OnFail`
          _))
      (`self.Reset Attack Rand`)
      (else
        (`self.GoToPlayer`)))
    (else
      (`/Engine/EditorBlueprintResources/StandardMacros.DoOnce` false :!label _label
        (:`Completed`
          (if (== _returnvalue 0)
            (`self.FireProjectile` :!label _label_2)
            (elif (== _returnvalue 100)
              (goto _label_2)
              (else
                (`self.Reset Attack Rand`)))))))))

(fn `UserConstructionScript`
  (`parent.UserConstructionScript`))