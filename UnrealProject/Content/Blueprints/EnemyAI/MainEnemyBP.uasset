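; Main enemy actor that takes its stats, name and mesh from the EnemyAIDataTable row matching its EnemyType.
; BeginPlay initializes the health HUD and hidden target selector, which bobs on a timeline.
; Hits subtract projectile damage or damage the player.
; Attack briefly binds OnActorHit, so player contact lowers health, reveals the HUD, and either destroys the enemy or knocks it back via timeline.
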(event `self.ReceiveBeginPlay`
  ;[1 1 1] Sets Enemy Stats Also sets target visibliity - Drew
  (bind _output_get (set `self.RowEnemyType` (`|GetEnumeratorNameAsString` (`self.EnemyType`))))
  (bind _returnvalue (`|GetDataTableRow` "/Game/Blueprints/EnemyAI/EnemyAIDataTable.EnemyAIDataTable" (`KismetStringLibrary.Conv_StringToName` _output_get))
    (:`then`
      (bind _output_get_2 (set `self.MaxHealth` (`.Health_10_78715AE74E29DA98E0C9818189E8272A` (break `/Game/Blueprints/EnemyAI/EnemyAIStruct` _returnvalue))))
      (set `self.Health` _output_get_2)
      (set `self.Damage` (`.Damage_8_4FE8259C49309BDD16E9089F6AC7774A` (break `/Game/Blueprints/EnemyAI/EnemyAIStruct` _returnvalue)))
      (set `self.Range` (`.Range_12_CAFF4F1A4F780CC97FA7B8A9F78FD715` (break `/Game/Blueprints/EnemyAI/EnemyAIStruct` _returnvalue)))
      (bind _asenemy_hud (cast `/Game/Blueprints/UI/EnemyHuds/EnemyHud` (`WidgetComponent.GetUserWidgetObject` (`self.EnemyHud`))))
      (bind _output_get_3 (set `/Game/Blueprints/UI/EnemyHuds/EnemyHud.MaxHealth` (`self.MaxHealth`) _asenemy_hud))
      (set `/Game/Blueprints/UI/EnemyHuds/EnemyHud.Health` _output_get_3 _asenemy_hud)
      (set `/Game/Blueprints/UI/EnemyHuds/EnemyHud.EnemyName` (`.Name_18_1216690343B8C32DF4B112B8B8B732BE` (break `/Game/Blueprints/EnemyAI/EnemyAIStruct` _returnvalue)) _asenemy_hud)
      (`StaticMeshComponent.SetStaticMesh` (`self.EnemyStaticMesh`) (break `/Game/Blueprints/EnemyAI/EnemyAIStruct` _returnvalue))
      (`SceneComponent.SetVisibility` (`self.TargetSelecter`) false false)
      (`|ExecutionSequence`
        (:`then_0`
          ;[1 1 1] Bounces The Target Selecter(Up/Down) - Drew
          (bind (_direction _newtrack_1) (`Timeline|Bounce` :!label _label)
            (:`Update`
              (`SceneComponent.K2_SetRelativeLocation` (`self.TargetSelecter`) _newtrack_1 false false)
              (`KismetSystemLibrary.Delay` 4.0)
              (goto _label :!via `PlayFromStart`))))
        (:`then_1`
          (`SceneComponent.SetVisibility` (`self.EnemyHud`) false false))))))

(event `self.ReceiveHit`
  (params (MyComp :type "PrimitiveComponent Object Reference") (Other :type "Actor Object Reference") (OtherComp :type "PrimitiveComponent Object Reference") (bSelfMoved :type Boolean) (HitLocation :type "Vector Structure") (HitNormal :type "Vector Structure") (NormalImpulse :type "Vector Structure") (Hit :type "HitResult Structure (by ref)"))
  ;[1 1 1] Enemy hit by projectile - Patrick Devine
  (bind _asbp_projectile (cast `/Game/Blueprints/BP_Projectile` Other)
    (:`then`
      (bind _output_get (set `self.Health` (- (`self.Health`) (`/Game/Blueprints/BP_Projectile.Damage` _asbp_projectile))))
      (if (<= _output_get 0.0)
        (`self.K2_DestroyActor`)))
    (:`CastFailed`
      ;[1 1 1] Enemy hits player - Patrick Devine
      (bind _asbp_player (cast `/Game/Blueprints/Character/BP_Player` Other))
      (`GameplayStatics.ApplyDamage` _asbp_player (`self.Damage`) null self))))

(event `/Game/Blueprints/IF_PlayerAttack.Attack`
  (params (Damage :type "Float (single-precision)") (OtherActorRightVector :type "Vector Structure"))
  ;[1 1 1] Enemy hit by player - Patrick Devine - Drew
  (add `self.OnActorHit` (delegate `ActorHit`))
  (`KismetSystemLibrary.Delay` 0.5)
  (remove `self.OnActorHit` (delegate `ActorHit`)))

(event `ActorHit` :!signature `self.OnActorHit`
  (params (SelfActor :type "Actor Object Reference") (OtherActor :type "Actor Object Reference") (NormalImpulse :type "Vector Structure") (Hit :type "HitResult Structure (by ref)"))
  ;[1 1 1] Enemy hit by player - Patrick Devine - Drew
  (cast `/Game/Blueprints/Character/BP_Player` OtherActor)
  (bind _asenemy_hud (cast `/Game/Blueprints/UI/EnemyHuds/EnemyHud` (`WidgetComponent.GetUserWidgetObject` (`self.EnemyHud`))))
  (set `/Game/Blueprints/UI/EnemyHuds/EnemyHud.Health` (- (`self.Health`) (stale `/Game/Blueprints/IF_PlayerAttack.Attack` Damage)) _asenemy_hud)
  ;;[1 1 1] Sets Enemy Health Visible when hit - Drew
  (`SceneComponent.SetVisibility` (`self.EnemyHud`) true false)
  (bind _output_get (set `self.Health` (- (`self.Health`) (stale `/Game/Blueprints/IF_PlayerAttack.Attack` Damage))))
  (if (<= _output_get 0.0)
    (`self.K2_DestroyActor`)
    (else
      (bind (_direction _move) (`Timeline|MoveActor` :!via `PlayFromStart`)
        (:`Update`
          (`self.K2_SetActorRelativeLocation` (+ (* _move (* (stale `/Game/Blueprints/IF_PlayerAttack.Attack` OtherActorRightVector) (`self.Knockback`))) (`self.K2_GetActorLocation`)) true))))))

(fn `UserConstructionScript`)