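; Bouncing cactus enemy that visually rolls while it moves, extending parent enemy behavior.
; Each tick compares location to the previous frame, spinning actor pitch while moving and resetting it upright when still, preserving yaw.
; The spin advances by a fixed per-frame increment, not scaled by delta time.
; Tick also pins TargetSelecter to the capsule's base with zero world rotation, so it ignores the roll.
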(event `self.ReceiveBeginPlay`
  (`parent.ReceiveBeginPlay`)
  (set `self.OldPos` (`self.K2_GetActorLocation`)))

(event `self.ReceiveTick`
  (params (DeltaSeconds :type "Float (single-precision)"))
  (bind (_returnvalue_x _returnvalue_y _returnvalue_z) (`KismetMathLibrary.BreakVector` (`self.K2_GetActorLocation`)))
  ;[1 1 1] Cactus move - Patrick Devine
  (`SceneComponent.K2_SetWorldLocationAndRotation` :`self` (`self.TargetSelecter`) :`NewLocation` (`KismetMathLibrary.MakeVector` _returnvalue_x _returnvalue_y (- _returnvalue_z (`.OutHalfHeight` (`CapsuleComponent.GetScaledCapsuleSize` (`self.CapsuleComponent`))))))
  (`self.Parent Tick`)
  (`|ExecutionSequence`
    (:`then_0`
      (if (not (== (`self.OldPos`) (`self.K2_GetActorLocation`)))
        (`self.Roll`)
        (else
          (`self.StopRolling`))))
    (:`then_1`
      (set `self.OldPos` (`self.K2_GetActorLocation`)))))

(event `Roll`
  (bind (_returnvalue_roll _returnvalue_pitch _returnvalue_yaw) (`KismetMathLibrary.BreakRotator` (`self.K2_GetActorRotation`)))
  (bind _yrotation (`self.YRotation`))
  ;[1 1 1] Rolls cactus on move - Patrick Devine
  (`self.K2_SetActorRotation` (`KismetMathLibrary.MakeRotator` 0.0 (- 360.0 (`self.YRotation`)) _returnvalue_yaw))
  (set `self.YRotation` (+ (`self.YIncrement`) _yrotation))
  (if (>= _yrotation 360.0)
    (set `self.YRotation` 0.0)))

(event `StopRolling`
  (bind (_returnvalue_roll _returnvalue_pitch _returnvalue_yaw) (`KismetMathLibrary.BreakRotator` (`self.K2_GetActorRotation`)))
  ;[1 1 1] Rolls cactus on move - Patrick Devine
  (`self.K2_SetActorRotation` (`KismetMathLibrary.MakeRotator` 0.0 0.0 _returnvalue_yaw)))

(fn `UserConstructionScript`
  (`parent.UserConstructionScript`))