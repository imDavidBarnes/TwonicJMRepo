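; Base enemy pawn for all enemy types, loading stats from a data table by type and driving an overhead health HUD.
; Snake and Cactus patrol and chase sighted players; Tick faces the player and randomly triggers timeline lunges in range.
; Attack briefly binds overlap for melee hits, causing invulnerability, stagger and knockback, or death with drops and poof.
; Bomb and looping fire damage reduce health separately, without a death check.
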(event `CreateHUD`
  ;[1 0.1131 0.8487] Create HUD - Drew
  (bind _asenemy_hud (cast `/Game/Blueprints/UI/EnemyHuds/EnemyHud` (`WidgetComponent.GetUserWidgetObject` (`self.EnemyHud`))))
  (bind _output_get (set `/Game/Blueprints/UI/EnemyHuds/EnemyHud.MaxHealth` (`self.MaxHealth`) _asenemy_hud))
  (set `/Game/Blueprints/UI/EnemyHuds/EnemyHud.Health` _output_get _asenemy_hud)
  (switch `/Game/Blueprints/EnemyAI/EnemyAIEnum` (`self.EnemyType`)
    (:`NewEnumerator0`
      (set `/Game/Blueprints/UI/EnemyHuds/EnemyHud.EnemyName` "Snake" _asenemy_hud))
    (:`NewEnumerator1`
      (set `/Game/Blueprints/UI/EnemyHuds/EnemyHud.EnemyName` "Cactus" _asenemy_hud))
    (:`NewEnumerator2`
      (set `/Game/Blueprints/UI/EnemyHuds/EnemyHud.EnemyName` "Piranha" _asenemy_hud))
    (:`NewEnumerator3`
      (set `/Game/Blueprints/UI/EnemyHuds/EnemyHud.EnemyName` "Ranged Cactus" _asenemy_hud))
    (:`NewEnumerator4`
      (set `/Game/Blueprints/UI/EnemyHuds/EnemyHud.EnemyName` "Anubis" _asenemy_hud))
    (:`NewEnumerator5`
      (set `/Game/Blueprints/UI/EnemyHuds/EnemyHud.EnemyName` "Ghost" _asenemy_hud)))
  (`SceneComponent.SetVisibility` (`self.TargetSelecter`) false false)
  (`|ExecutionSequence`
    (:`then_0`
      ;;[1 0.1131 0.8487] Bounces The Target Selecter(Up/Down) - Drew
      (bind (_direction _newtrack_1) (`Timeline|Timeline_0` :!label _label)
        (:`Update`
          (`SceneComponent.K2_SetRelativeLocation` (`self.TargetSelecter`) _newtrack_1 false false)
          (`KismetSystemLibrary.Delay` 4.0)
          (goto _label :!via `PlayFromStart`))))
    (:`then_1`
      (`SceneComponent.SetVisibility` (`self.EnemyHud`) false false))))

(event `SetMaterial`
  (params (Mat :type "MaterialInterface Object Reference"))
  (bind _output_get (set `self.EnemyMat` Mat))
  (`PrimitiveComponent.SetMaterial` (`self.Mesh`) 0 _output_get))

(event `self.ReceiveBeginPlay`
  ;[1 0.1131 0.8487] Sets Enemy Stats Also sets target visibliity - Drew
  (`self.SetMaterial` "/Game/Mannequin/Character/Materials/M_Male_Body.M_Male_Body")
  (`|ExecutionSequence`
    (:`then_0`
      (bind _output_get (set `self.RowEnemyType` (`|GetEnumeratorNameAsString` (`self.EnemyType`))))
      (bind _returnvalue (`|GetDataTableRow` "/Game/Blueprints/EnemyAI/EnemyAIDataTable.EnemyAIDataTable" (`KismetStringLibrary.Conv_StringToName` _output_get))
        (:`then`
          (bind _output_get_2 (set `self.MaxHealth` (`.Health_10_78715AE74E29DA98E0C9818189E8272A` (break `/Game/Blueprints/EnemyAI/EnemyAIStruct` _returnvalue))))
          (set `self.Health` _output_get_2)
          (set `AttackingEntity.Damage` (`.Damage_8_4FE8259C49309BDD16E9089F6AC7774A` (break `/Game/Blueprints/EnemyAI/EnemyAIStruct` _returnvalue)) (`self.AttackingEntity`))
          (set `self.Range` (`.Range_12_CAFF4F1A4F780CC97FA7B8A9F78FD715` (break `/Game/Blueprints/EnemyAI/EnemyAIStruct` _returnvalue)))
          (`self.CreateHUD`))))
    (:`then_1`
      (`self.Start Patroling`))))

(event `Invulnerability`
  (params (Duration :type "Float (double-precision)"))
  ;[1 0.2262 0.1864] Call this to make Enemy invulnerable - Patrick Devine
  (set `self.CanHit` false)
  (`KismetSystemLibrary.Delay` Duration)
  (set `self.CanHit` true))

(event `ActorHit`
  (params (SelfActor :type "Actor Object Reference") (OtherActor :type "Actor Object Reference") (NormalImpulse :type "Vector Structure") (Hit :type "HitResult Structure (by ref)"))
  ;[1 0.2262 0.1864] Enemy hit by player - Patrick Devine - Drew
)

(event `/Game/Blueprints/IF_PlayerAttack.Attack`
  (params (Damage :type "Float (single-precision)") (OtherActorForwardVector :type "Vector Structure"))
  ;[1 0.2262 0.1864] Enemy hit by player - Patrick Devine - Drew
  (add `self.OnActorBeginOverlap` (delegate `ActorOverlap`))
  (`KismetSystemLibrary.Delay` 0.5)
  (remove `self.OnActorBeginOverlap` (delegate `ActorOverlap`)))

(event `self.ReceiveHit`
  (params (MyComp :type "PrimitiveComponent Object Reference") (Other :type "Actor Object Reference") (OtherComp :type "PrimitiveComponent Object Reference") (bSelfMoved :type Boolean) (HitLocation :type "Vector Structure") (HitNormal :type "Vector Structure") (NormalImpulse :type "Vector Structure") (Hit :type "HitResult Structure (by ref)"))
  ;[1 0.2262 0.1864] Enemy hit by projectile - Patrick Devine
  ;;[1 1 1] Use this to apply damage health to healthbars - Drew
  (`self.Parent Hit` Other))

(event `Parent Hit`
  (params (Other :type "Actor Object Reference"))
  ;[1 0.2262 0.1864] Enemy hit by projectile - Patrick Devine
  ;;[1 1 1] Use this to apply damage health to healthbars - Drew
  (`|ExecutionSequence`
    (:`then_0`
      (cast `/Game/Blueprints/BP_Projectile` Other))
    (:`then_1`
      ;[1 0.2262 0.1864] Enemy hits player - Patrick Devine
      (bind _asbp_player (cast `/Game/Blueprints/Character/BP_Player` Other))
      (bind _returnvalue (`AttackingEntity.GetAttackDamage` (`self.AttackingEntity`)))
      (`GameplayStatics.ApplyDamage` _asbp_player _returnvalue null self))
    (:`then_2`
      (`self.UpdateHealth`))))

(event `Stagger`
  (params (StaggerDuration :type "Float (double-precision)"))
  ;[1 0.2262 0.1864] Stun - Patrick Devine
  (`PrimitiveComponent.SetMaterial` (`self.Mesh`) 0 "/Game/Materials/Mat_EnemyHit.Mat_EnemyHit")
  (set `self.Staggered` true)
  (`KismetSystemLibrary.Delay` StaggerDuration)
  (set `self.Staggered` false)
  (`PrimitiveComponent.SetMaterial` (`self.Mesh`) 0 (`self.EnemyMat`)))

(event `ActorOverlap` :!signature `self.OnActorBeginOverlap`
  (params (OverlappedActor :type "Actor Object Reference") (OtherActor :type "Actor Object Reference"))
  ;[1 0.2262 0.1864] Enemy hit by player - Patrick Devine - Drew
  (if (`self.CanHit`)
    (cast `/Game/Blueprints/EquipItems/BP_MeleeWeapon` OtherActor)
    (bind _asenemy_hud (cast `/Game/Blueprints/UI/EnemyHuds/EnemyHud` (`WidgetComponent.GetUserWidgetObject` (`self.EnemyHud`))))
    (set `/Game/Blueprints/UI/EnemyHuds/EnemyHud.Health` (- (`self.Health`) (stale `/Game/Blueprints/IF_PlayerAttack.Attack` Damage)) _asenemy_hud)
    ;;[1 1 1] Sets Enemy Health Visible when hit - Drew
    (`SceneComponent.SetVisibility` (`self.EnemyHud`) true false)
    (`self.Invulnerability` 0.2)
    (bind _output_get (set `self.Health` (- (`self.Health`) (stale `/Game/Blueprints/IF_PlayerAttack.Attack` Damage))))
    (if (<= _output_get 0.0)
      (`self.Death`)
      (else
        (`self.Stagger` 0.5)
        (bind (_direction _move) (`Timeline|TM_TakeDamage` :!via `PlayFromStart`)
          (:`Update`
            (`self.K2_SetActorRelativeLocation` (+ (`/Game/Blueprints/BP_MacroLib.DeltaTime` (`self.DeltaTime`) (* _move (* (stale `/Game/Blueprints/IF_PlayerAttack.Attack` OtherActorForwardVector) (`AttackingEntity.Knockback` (`self.AttackingEntity`))))) (`self.K2_GetActorLocation`)) true))
          (:`Finished`
            (set `self.CanSee` true)))))))

(event `UpdateHealth`
  ;[1 0.2262 0.1864] Update Health - Drew
  (bind _asenemy_hud (cast `/Game/Blueprints/UI/EnemyHuds/EnemyHud` (`WidgetComponent.GetUserWidgetObject` (`self.EnemyHud`))))
  (set `/Game/Blueprints/UI/EnemyHuds/EnemyHud.Health` (`self.Health`) _asenemy_hud)
  (if (<= (`self.Health`) 0.0)
    (`self.K2_DestroyActor`)))

(event `SpawnMana`
  ;[1 0.2262 0.1864] Spawn Pickups - Patrick Devine
  (if (`KismetMathLibrary.RandomBoolWithWeight` 0.2)
    (bind _returnvalue (`|SpawnActorFromClass` "/Game/Blueprints/Interactables/Pickups/BP_ManaDrop.BP_ManaDrop_C" (`KismetMathLibrary.MakeTransform` (`self.K2_GetActorLocation`) (`KismetMathLibrary.MakeRotator` 0.0 0.0 (* (`KismetMathLibrary.RandomFloat`) 360.0)) (0.5 0.5 0.5)) "AdjustIfPossibleButAlwaysSpawn" "OverrideRootScale" null null))
    (set `Pickup.quantity` 10 _returnvalue)))

(event `Below Level`
  (bind (_returnvalue_x _returnvalue_y _returnvalue_z) (`KismetMathLibrary.BreakVector` (`self.K2_GetActorLocation`)))
  ;[0.2183 1 0.1567] If enemy goes below level, destroy actor - Patrick Devine
  (if (< _returnvalue_z (`self.BelowLevelZ`))
    (`self.K2_DestroyActor`)))

(event `Face Player`
  (bind (_returnvalue_roll _returnvalue_pitch) (`KismetMathLibrary.BreakRotator` (`self.K2_GetActorRotation`)))
  ;[0.2183 1 0.1567] Face Player - Patrick Devine
  (if (`self.CanSee`)
    (bind _asbp_player (cast `/Game/Blueprints/Character/BP_Player` (`GameplayStatics.GetPlayerPawn` 0)))
    (bind (_returnvalue_roll_2 _returnvalue_pitch_2 _returnvalue_yaw) (`KismetMathLibrary.BreakRotator` (`KismetMathLibrary.FindLookAtRotation` (`self.K2_GetActorLocation`) (`self.K2_GetActorLocation` _asbp_player))))
    (`self.K2_SetActorRotation` (`KismetMathLibrary.MakeRotator` _returnvalue_roll _returnvalue_pitch _returnvalue_yaw))))

(event `SpawnHealth`
  ;[1 0.2262 0.1864] Spawn Pickups - Patrick Devine
  (if (`KismetMathLibrary.RandomBoolWithWeight` 0.4)
    (bind _returnvalue (`|SpawnActorFromClass` "/Game/Blueprints/Interactables/Pickups/BP_HealthDrop.BP_HealthDrop_C" (`KismetMathLibrary.MakeTransform` (`self.K2_GetActorLocation`) (`KismetMathLibrary.MakeRotator` 0.0 0.0 (* (`KismetMathLibrary.RandomFloat`) 360.0)) (0.5 0.5 0.5)) "AdjustIfPossibleButAlwaysSpawn" "OverrideRootScale" null null))
    (set `Pickup.quantity` 10 _returnvalue)))

(event `EnemyAttack`
  (params (ToPlayer :type "Vector Structure") (Scale :type "Float (double-precision)"))
  ;[1 0.2262 0.1864] Attack - Patrick Devine
  (if (not (`self.Staggered`))
    (`KismetSystemLibrary.PrintString` "")
    (set `self.IsAttacking` true)
    (bind (_direction _move) (`Timeline|TM_Attack` :!via `PlayFromStart`)
      (:`Update`
        (bind _returnvalue (+ (`/Game/Blueprints/BP_MacroLib.DeltaTime` (`self.DeltaTime`) (* _move (* (`KismetMathLibrary.Normal` ToPlayer) (* Scale (`self.Range`))))) (`self.K2_GetActorLocation`)))
        (bind (_sweephitresult _returnvalue_2) (`self.K2_SetActorLocation` _returnvalue true))
        (`KismetSystemLibrary.PrintString` (`KismetStringLibrary.Conv_BoolToString` _returnvalue_2))
        (set `self.OldPos` _returnvalue))
      (:`Finished`
        (set `self.IsAttacking` false)))))

(event `SpawnDrops`
  ;[1 0.2262 0.1864] Spawn Pickups - Patrick Devine
  (`self.SpawnMoney`)
  (`self.SpawnHealth`)
  (`self.SpawnMana`))

(event `self.PawnSensing.OnSeePawn`
  (params (Pawn :type "Pawn Object Reference"))
  ;[0.2183 1 0.1567] Simple AI Move to actors location - Drew
  (if (not (`self.Staggered`))
    (switch `/Game/Blueprints/EnemyAI/EnemyAIEnum` (`self.EnemyType`)
      (:`NewEnumerator0`
        (bind _asbp_player (cast `/Game/Blueprints/Character/BP_Player` Pawn :!label _label_2))
        (set `self.CanSee` true)
        (if (`self.InRange`)
          (`|AIMoveTo` self (`self.K2_GetActorLocation`) null)
          (else
            (set `self.IsOnPatrol?` false)
            (`|AIMoveTo` self (0.0 0.0 0.0) _asbp_player
              (:`OnSuccess`
                (set `self.IsOnPatrol?` true))))))
      (:`NewEnumerator1`
        (goto _label_2))
      (:`NewEnumerator2`
        (set `self.CanSee` true :!label _label_3))
      (:`NewEnumerator3`
        (goto _label_3))
      (:`NewEnumerator4`
        (goto _label_3)))))

(event `Death`
  ;[1 0.2262 0.1864] Enemy death - Patrick Devine
  (`self.SetActorEnableCollision` false)
  (set `self.Staggered` true)
  (`SceneComponent.SetVisibility` (`self.EnemyHud`) false false)
  (`self.SpawnDrops`)
  (`self.DeathAffectPlay`))

(event `AttackSense`
  (params (Range :type "Float (double-precision)"))
  ;[1 0.2262 0.1864] Attacks when close enough - Patrick Devine
  (if (`self.CanSee`)
    (bind _toplayer (`self.GetToPlayer`))
    (set `self.InRange` (<= (`KismetMathLibrary.VSize` _toplayer) Range))))

(event `Start Patroling`
  ;[0.2183 1 0.1567] Simple Patrol Randomly Around Area - Drew
  (if (not (`self.Staggered`))
    (switch `/Game/Blueprints/EnemyAI/EnemyAIEnum` (`self.EnemyType`)
      (:`NewEnumerator0`
        _)
      (:`NewEnumerator1`
        _))
    (if (`self.InRange`)
      _
      (elif (`self.IsOnPatrol?`)
        (`|AIMoveTo` self (`NavigationSystemV1.K2_GetRandomReachablePointInRadius` (`self.K2_GetActorLocation`) 5000.0 null null) null
          (:`OnSuccess`
            (`KismetSystemLibrary.Delay` 2.0)
            (`self.Start Patroling`)))))))

(event `SpawnMoney`
  ;[1 0.2262 0.1864] Spawn money in a 360 degree circle around enemy (distributed) on death - Patrick Devine
  (for _index (range (+ (`self.MoneyDropAmount`) 1))
    (bind _returnvalue (`|SpawnActorFromClass` "/Game/Blueprints/Interactables/Pickups/BP_Coin.BP_Coin_C" (`KismetMathLibrary.MakeTransform` (`self.K2_GetActorLocation`) (`KismetMathLibrary.MakeRotator` 0.0 0.0 (* _index (/ 360.0 (`KismetMathLibrary.Conv_IntToDouble` (`self.MoneyDropAmount`))))) (0.25 0.25 0.25)) "AdjustIfPossibleButAlwaysSpawn" "OverrideRootScale" null null))
    (set `Pickup.quantity` 1 _returnvalue)))

(event `Parent Tick`
  (params (DeltaTime :type "Float (double-precision)"))
  ;[1 0.1131 0.8487] Parent tick - Patrick Devine
  (`|ExecutionSequence`
    (:`then_0`
      (set `self.DeltaTime` DeltaTime)
      (`self.AttackSense` (`self.Range`))
      (`self.Face Player`))
    (:`then_1`
      (if (== (`KismetMathLibrary.RandomIntegerInRange` 0 500) 0)
        (if (`self.InRange`)
          (bind _asbp_player (cast `/Game/Blueprints/Character/BP_Player` (`GameplayStatics.GetPlayerPawn` 0)))
          (`self.EnemyAttack` (- (`self.K2_GetActorLocation` _asbp_player) (`self.K2_GetActorLocation`)) 1.0))))))

(event `ExplosionDamage`
  ;[1 0.2262 0.1864] Explosion Enemy Damage - Drew
  (bind _output_get (set `self.Health` (- (stale _output_get) (`KismetMathLibrary.Conv_IntToDouble` (`KismetMathLibrary.RandomIntegerInRange` 38 65)))))
  (bind _asenemy_hud (cast `/Game/Blueprints/UI/EnemyHuds/EnemyHud` (`WidgetComponent.GetUserWidgetObject` (`self.EnemyHud`))))
  (set `/Game/Blueprints/UI/EnemyHuds/EnemyHud.Health` _output_get _asenemy_hud))

(event `FireDMG`
  (params (`Bomb Ref` :type "Actor Object Reference"))
  ;[1 0.2262 0.1864] Fire Enemy Damage - Drew
  (set `self.OnFire` true)
  (`KismetSystemLibrary.K2_SetTimerDelegate` (delegate `Fire`) 1.0 (`self.OnFire`) :!label _label_4))

(event `DeathAffectPlay`
  ;[1 0.2262 0.1864] Spawn poof and shrink self on death then destroy actor - Patrick Devine
  (bind (_direction _scale) (`Timeline|Die` :!via `PlayFromStart`)
    (:`Update`
      (`self.SetActorScale3D` _scale))
    (:`Finished`
      (`SceneComponent.SetHiddenInGame` (`self.Mesh`) true false)
      (`self.SetActorScale3D` (1.0 1.0 1.0))
      (`self.StartPoof`)
      (`KismetSystemLibrary.Delay` 2.5)
      (`ActorComponent.K2_DestroyComponent` (stale `StartPoof` _returnvalue))
      (`self.K2_DestroyActor`))))

(event `DelayAttack`
  (params (DelayTime :type "Float (double-precision)"))
  (`KismetSystemLibrary.Delay` (* DelayTime (`KismetMathLibrary.RandomFloat`))))

(event `StartPoof`
  ;[1 0.2262 0.1864] Spawn poof and shrink self on death then destroy actor - Patrick Devine
  (bind _returnvalue (`NiagaraFunctionLibrary.SpawnSystemAtLocation` "/Game/VFX/N_Poof.N_Poof" (`self.K2_GetActorLocation`) (`self.K2_GetActorRotation`))))

(event `Fire`
  ;[1 0.2262 0.1864] Fire Enemy Damage - Drew
  (`/Engine/EditorBlueprintResources/StandardMacros.IsValid` (stale `FireDMG` `Bomb Ref`)
    (:`Is Valid`
      (`self.DamageWithBomb`))
    (:`Is Not Valid`
      (set `self.OnFire` false)
      (goto _label_4))))

(event `self.ReceiveTick`
  (params (DeltaSeconds :type "Float (single-precision)"))
  (if (not (`self.Staggered`))
    (`self.Parent Tick` DeltaSeconds)))

(event `Disable Fire`
  ;[1 0.2262 0.1864] Fire Enemy Damage - Drew
  (set `self.OnFire` false)
  (goto _label_4))

(event `DirectHitWithBomb`
  (`self.DamageWithBomb`))

(fn `DamageWithBomb`
  (bind _output_get (set `self.Health` (- (stale _output_get) (`KismetMathLibrary.Conv_IntToDouble` (`KismetMathLibrary.RandomIntegerInRange` 3 7)))))
  (bind _asenemy_hud (cast `/Game/Blueprints/UI/EnemyHuds/EnemyHud` (`WidgetComponent.GetUserWidgetObject` (`self.EnemyHud`))))
  (set `/Game/Blueprints/UI/EnemyHuds/EnemyHud.Health` _output_get _asenemy_hud))

(fn `GetToPlayer`
  (returns (ToPlayer :type "Vector Structure"))
  (bind _asbp_player (cast `/Game/Blueprints/Character/BP_Player` (`GameplayStatics.GetPlayerPawn` 0)))
  (return (- (`self.K2_GetActorLocation` _asbp_player) (`self.K2_GetActorLocation`))))

(fn `SetDifficultyValues`
  (params (DamageMultiplier :type "Float (double-precision)") (HealthMultiplier :type "Float (double-precision)") (Material :type "MaterialInterface Object Reference"))
  (set `AttackingEntity.Damage` DamageMultiplier (`self.AttackingEntity`))
  (bind _output_get (set `self.Health` HealthMultiplier))
  (set `self.MaxHealth` _output_get)
  (set `self.EnemyMat` Material))

(fn `UserConstructionScript`)