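; Sliding gate actor that moves its door out of the way when the player overlaps its collision volume.
; The construction script caches the world location of the Movement component as the end position.
; On overlap by BP_Player, a short delay precedes setting the door component to that position in one unswept jump, with no interpolation.
; BeginPlay stores the start position, but nothing shown uses it to close the gate.
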(event `self.ReceiveBeginPlay`
  ;[1 1 1] Condition for movement
  (set `self.Start Position` (`self.K2_GetActorLocation`)))

(event `self.Gate Collision.OnComponentBeginOverlap`
  (params (OverlappedComponent :type "PrimitiveComponent Object Reference") (OtherActor :type "Actor Object Reference") (OtherComp :type "PrimitiveComponent Object Reference") (OtherBodyIndex :type Integer) (bFromSweep :type Boolean) (SweepResult :type "HitResult Structure (by ref)"))
  ;[1 1 1] Collision with Player
  (if true
    (cast `/Game/Blueprints/Character/BP_Player` OtherActor)
    ;[1 1 1] Door Sliding
    (`KismetSystemLibrary.Delay` 0.5)
    (`SceneComponent.K2_SetWorldLocation` (`self.Gate-Door Appearance`) (`self.End Position`) false false)))

(fn `UserConstructionScript`
  ;[1 1 1] Move To
  (set `self.End Position` (`SceneComponent.K2_GetComponentLocation` (`self.Movement`))))