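; Pressure pad gate actor that opens a gate when BP_Player steps into its PressureArea.
; The construction script caches target world locations from the Movement and GateMovement marker components.
; On overlap, the plate snaps to its target after a short delay and the gate after a longer one, without interpolation.
; Nothing resets either piece; the start position saved on BeginPlay is never used.
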(event `self.ReceiveBeginPlay`
  ;[1 1 1] Beginning Location
  (set `self.Start Position` (`self.K2_GetActorLocation`)))

(event `self.Pressure Area.OnComponentBeginOverlap`
  (params (OverlappedComponent :type "PrimitiveComponent Object Reference") (OtherActor :type "Actor Object Reference") (OtherComp :type "PrimitiveComponent Object Reference") (OtherBodyIndex :type Integer) (bFromSweep :type Boolean) (SweepResult :type "HitResult Structure (by ref)"))
  ;[1 1 1] Collision
  (cast `/Game/Blueprints/Character/BP_Player` OtherActor)
  (`|ExecutionSequence`
    (:`then_0`
      ;[1 1 1] Pressure Pad Movement
      (`KismetSystemLibrary.Delay` 0.2)
      (`SceneComponent.K2_SetWorldLocation` (`self.Pressure Plate`) (`self.End Position1`) false false))
    (:`then_1`
      ;[1 1 1] Gate Movement
      (`KismetSystemLibrary.Delay` 2.0)
      (`SceneComponent.K2_SetWorldLocation` (`self.Gate Appearance`) (`self.End Position`) false false))))

(fn `Pressure Pad Movement`
  ;[1 1 1] Pressure Pad Movement
  (set `self.End Position1` (`SceneComponent.K2_GetComponentLocation` (`self.Movement`))))

(fn `UserConstructionScript`
  ;[1 1 1] End Location
  (`|ExecutionSequence`
    (:`then_0`
      (set `self.End Position1` (`SceneComponent.K2_GetComponentLocation` (`self.Movement`))))
    (:`then_1`
      (set `self.End Position` (`SceneComponent.K2_GetComponentLocation` (`self.Gate Movement`))))))