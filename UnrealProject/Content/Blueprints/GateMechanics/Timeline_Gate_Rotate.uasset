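; Gate actor that swings its door open by rotation the first time the player enters its collision volume.
; A BP_Player overlap on GateCollision passes a DoOnce and plays the GateOpen timeline.
; Each timeline update adds the DoorRotation value to the door's relative yaw, so rotation accumulates rather than being set absolutely.
; The gate never closes; leftover door-sliding nodes are disconnected.
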(event `self.ReceiveBeginPlay`
  ;[1 1 1] Condition for movement
)

(event `self.Gate Collision.OnComponentBeginOverlap`
  (params (OverlappedComponent :type "PrimitiveComponent Object Reference") (OtherActor :type "Actor Object Reference") (OtherComp :type "PrimitiveComponent Object Reference") (OtherBodyIndex :type Integer) (bFromSweep :type Boolean) (SweepResult :type "HitResult Structure (by ref)"))
  ;[1 1 1] Collision with Player
  (cast `/Game/Blueprints/Character/BP_Player` OtherActor)
  (`/Engine/EditorBlueprintResources/StandardMacros.DoOnce` false
    (:`Completed`
      ;[1 1 1] Timeline
      (bind (_direction _door_rotation) (`Timeline|Gate Open` :`NewTime` 2.0)
        (:`Update`
          ;[1 1 1] Rotation
          (`|ExecutionSequence`
            (:`then_0`
              (`SceneComponent.K2_AddRelativeRotation` (`self.Gate-Door Appearance`) (`KismetMathLibrary.MakeRotator` 0.0 0.0 _door_rotation) false false))))))))

(event `self.Gate Collision.OnComponentEndOverlap`
  (params (OverlappedComponent :type "PrimitiveComponent Object Reference") (OtherActor :type "Actor Object Reference") (OtherComp :type "PrimitiveComponent Object Reference") (OtherBodyIndex :type Integer))
  ;[1 1 1] Collision with Player
)

(fn `UserConstructionScript`
  ;[1 1 1] Move To
)