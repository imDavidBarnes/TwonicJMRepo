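; BP_Vase is a breakable overworld vase that drops coins when it is broken.
; BreakObject calls SpawnMoney and then destroys the actor.
; SpawnMoney spawns MoneyDropAmount small BP_Coin actors of quantity one above the vase, yawed at even intervals around a full circle.
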(event `self.BreakObject`
  ;[1 1 1] Vase break - Patrick Devine
  (`self.SpawnMoney`)
  (`self.K2_DestroyActor`))

(event `SpawnMoney`
  (bind (_returnvalue_x _returnvalue_y _returnvalue_z) (`KismetMathLibrary.BreakVector` (`self.K2_GetActorLocation`)))
  ;[1 1 1] Vase break - Patrick Devine
  (for _index (range (`self.MoneyDropAmount`))
    (bind _returnvalue (`|SpawnActorFromClass` "/Game/Blueprints/Interactables/Pickups/BP_Coin.BP_Coin_C" (`KismetMathLibrary.MakeTransform` (`KismetMathLibrary.MakeVector` _returnvalue_x _returnvalue_y (+ _returnvalue_z (`self.ZPosOffset`))) (`KismetMathLibrary.MakeRotator` 0.0 0.0 (* _index (/ 360.0 (`KismetMathLibrary.Conv_IntToDouble` (`self.MoneyDropAmount`))))) (0.25 0.25 0.25)) "AdjustIfPossibleButAlwaysSpawn" "OverrideRootScale" null null))
    (set `Pickup.quantity` 1 _returnvalue)))

(fn `UserConstructionScript`)