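; BP_BreakableObject is an overworld object that destroys itself when hit by a strong enough melee weapon.
; Its Attack event binds an actor overlap handler, then unbinds it after a short delay, so hits only count during that window.
; The handler accepts only BP_MeleeWeapon actors and calls BreakObject when their AttackDamage meets the BreakSwordDamageNeeded threshold.
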(event `/Game/Blueprints/IF_PlayerAttack.Attack`
  (params (Damage :type "Float (single-precision)") (OtherActorForwardVector :type "Vector Structure"))
  (add `self.OnActorBeginOverlap` (delegate `ActorOverlap`))
  (`KismetSystemLibrary.Delay` 0.5)
  (remove `self.OnActorBeginOverlap` (delegate `ActorOverlap`)))

(event `ActorOverlap` :!signature `self.OnActorBeginOverlap`
  (params (OverlappedActor :type "Actor Object Reference") (OtherActor :type "Actor Object Reference"))
  (bind _asbp_melee_weapon (cast `/Game/Blueprints/EquipItems/BP_MeleeWeapon` OtherActor))
  (if (>= (`MeleeWeapon.AttackDamage` _asbp_melee_weapon) (`self.BreakSwordDamageNeeded`))
    (`self.BreakObject`)))

(event `BreakObject`
  (`self.K2_DestroyActor`))

(fn `UserConstructionScript`)