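; BP_Checkpoint is an interactable respawn checkpoint that sets the player's spawn position.
; Its collider enables input from player controller 0 while BP_Player overlaps it and disables input on exit.
; Pressing Interact stores the Spawn component's world location in the player's SpawnPos and prints a confirmation.
; A DoOnce gate, reset when the player leaves, limits this to one activation per visit.
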(event `self.Collider.OnComponentBeginOverlap`
  (params (OverlappedComponent :type "PrimitiveComponent Object Reference") (OtherActor :type "Actor Object Reference") (OtherComp :type "PrimitiveComponent Object Reference") (OtherBodyIndex :type Integer) (bFromSweep :type Boolean) (SweepResult :type "HitResult Structure (by ref)"))
  ;[1 1 1] Allows the checkpoint to read input when overlapped - Kieran Ganner
  (cast `/Game/Blueprints/Character/BP_Player` OtherActor)
  (`self.EnableInput` (`GameplayStatics.GetPlayerController` 0)))

(event `self.Collider.OnComponentEndOverlap`
  (params (OverlappedComponent :type "PrimitiveComponent Object Reference") (OtherActor :type "Actor Object Reference") (OtherComp :type "PrimitiveComponent Object Reference") (OtherBodyIndex :type Integer))
  ;[1 1 1] Allows the checkpoint to read input when overlapped - Kieran Ganner
  (cast `/Game/Blueprints/Character/BP_Player` OtherActor)
  (`self.DisableInput` (`GameplayStatics.GetPlayerController` 0))
  (goto _label :!via `Reset`))

(event `InputAction|Interact`
  (params (Key :type "Key Structure"))
  ;[1 1 1] Sets player spawn to location of checkpoint when interacts with - Kieran Ganner
  (:`Pressed`
    (`/Engine/EditorBlueprintResources/StandardMacros.DoOnce` false :!label _label
      (:`Completed`
        (bind _asbp_player (cast `/Game/Blueprints/Character/BP_Player` (`GameplayStatics.GetPlayerCharacter` 0)))
        (set `/Game/Blueprints/Character/BP_Player.SpawnPos` (`SceneComponent.K2_GetComponentLocation` (`self.Spawn`)) _asbp_player)
        (`KismetSystemLibrary.PrintString` "Spawnpoint Set")))))

(fn `UserConstructionScript`)