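; BP_Elevator is an elevator that the player raises or lowers by interacting while inside its trigger box.
; Overlap by BP_Player enables input, and pressing Interact plays the Elevator timeline.
; Leaving the box disables input and reverses the timeline, returning the platform toward its start.
; The timeline sets the cube's relative Z from its Move track times a multiplier, at a play rate set on BeginPlay.
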(event `self.Box.OnComponentBeginOverlap`
  (params (OverlappedComponent :type "PrimitiveComponent Object Reference") (OtherActor :type "Actor Object Reference") (OtherComp :type "PrimitiveComponent Object Reference") (OtherBodyIndex :type Integer) (bFromSweep :type Boolean) (SweepResult :type "HitResult Structure (by ref)"))
  ;[1 1 1] Allows the elevator to read input when overlapped - Kieran Ganner
  (cast `/Game/Blueprints/Character/BP_Player` OtherActor)
  (`self.EnableInput` (`GameplayStatics.GetPlayerController` 0)))

(event `self.Box.OnComponentEndOverlap`
  (params (OverlappedComponent :type "PrimitiveComponent Object Reference") (OtherActor :type "Actor Object Reference") (OtherComp :type "PrimitiveComponent Object Reference") (OtherBodyIndex :type Integer))
  ;[1 1 1] Allows the elevator to read input when overlapped - Kieran Ganner
  (cast `/Game/Blueprints/Character/BP_Player` OtherActor)
  (`self.DisableInput` (`GameplayStatics.GetPlayerController` 0))
  ;[1 1 1] Moves elevator overtime - Kieran Ganner
  (bind (_direction _move) (`Timeline|Elevator` :!via `Reverse` :!label _label)
    (:`Update`
      (`SceneComponent.K2_SetRelativeLocation` (`self.Cube`) (`KismetMathLibrary.MakeVector` 0.0 0.0 (* _move (`self.VerticleMultiplicitive`))) false false))))

(event `self.ReceiveBeginPlay`
  ;[1 1 1] Sets speed of elevator - Kieran Ganner
  (`TimelineComponent.SetPlayRate` (`self.Elevator`) (`self.PlaybackRate`)))

(event `InputAction|Interact`
  (params (Key :type "Key Structure"))
  ;[1 1 1] Moves elevator overtime - Kieran Ganner
  (:`Pressed`
    (goto _label)))

(fn `UserConstructionScript`)