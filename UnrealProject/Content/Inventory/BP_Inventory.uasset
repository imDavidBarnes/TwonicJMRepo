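; BP_Inventory is an inventory actor that opens an inventory UI, with AddItem and RemoveItem still empty stubs.
; Tick polls IsShowing and uses a DoOnce with no reset wired, so the opening logic runs only once.
; That logic disables player character input and shows the mouse cursor.
; If PlayerRef is valid, it immediately re-enables input and adds InvenUI through the PlayerHUD.
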(event `self.ReceiveTick`
  (params (DeltaSeconds :type "Float (single-precision)"))
  (bind _returnvalue (`GameplayStatics.GetPlayerController` 0))
  (bind _returnvalue_2 (`GameplayStatics.GetPlayerCharacter` 0))
  (bind _returnvalue_3 (`GameplayStatics.GetPlayerController` 0))
  (if (`self.isShowing`)
    (`/Engine/EditorBlueprintResources/StandardMacros.DoOnce` false
      (:`Completed`
        (`self.DisableInput` _returnvalue_2 _returnvalue)
        (set `PlayerController.bShowMouseCursor` true _returnvalue)
        (`/Engine/EditorBlueprintResources/StandardMacros.IsValid` (`self.PlayerRef`)
          (:`Is Valid`
            (`self.EnableInput` _returnvalue_2 _returnvalue_3)
            (bind _asplayer_hud (cast `/Game/Blueprints/UI/PlayerHUD` (`PlayerController.GetHUD` _returnvalue_3)))
            (`/Game/Blueprints/UI/PlayerHUD.Add UI` _asplayer_hud (`self.InvenUI`))))))))

(fn `AddItem`)

(fn `RemoveItem`)

(fn `UserConstructionScript`)