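; Elevator actor that raises and lowers a cube platform through a timeline.
; Box overlap enables input on the Main_Character itself rather than the elevator; leaving disables that character's input and reverses the timeline.
; Pressing E prints a debug string and plays the timeline, with no overlap check of its own.
; Each timeline update sets the cube's relative Z from the Move track scaled by VerticleMultiplicitive.
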(event `self.Box.OnComponentBeginOverlap`
  (params (OverlappedComponent :type "PrimitiveComponent Object Reference") (OtherActor :type "Actor Object Reference") (OtherComp :type "PrimitiveComponent Object Reference") (OtherBodyIndex :type Integer) (bFromSweep :type Boolean) (SweepResult :type "HitResult Structure (by ref)"))
  ;[1 1 1] Allows the elevator to read input when overlapped - Kieran Ganner
  (bind _asmain_character (cast `/Game/Character/Main_Character` OtherActor))
  (`self.EnableInput` _asmain_character (`GameplayStatics.GetPlayerController` 0)))

(event `self.Box.OnComponentEndOverlap`
  (params (OverlappedComponent :type "PrimitiveComponent Object Reference") (OtherActor :type "Actor Object Reference") (OtherComp :type "PrimitiveComponent Object Reference") (OtherBodyIndex :type Integer))
  ;[1 1 1] Allows the elevator to read input when overlapped - Kieran Ganner
  (bind _asmain_character (cast `/Game/Character/Main_Character` OtherActor))
  (`self.DisableInput` _asmain_character (`GameplayStatics.GetPlayerController` 0))
  ;[1 1 1] Moves elevator overtime - Kieran Ganner
  (bind (_direction _move) (`Timeline|Elevator` :!via `Reverse` :!label _label)
    (:`Update`
      (`SceneComponent.K2_SetRelativeLocation` (`self.Cube`) (`KismetMathLibrary.MakeVector` 0.0 0.0 (* _move (`self.VerticleMultiplicitive`))) false false))))

(event `Key|E`
  (params (Key :type "Key Structure"))
  ;[1 1 1] Moves elevator overtime - Kieran Ganner
  (:`Pressed`
    (`KismetSystemLibrary.PrintString` "Hello")
    (goto _label)))

(fn `UserConstructionScript`)